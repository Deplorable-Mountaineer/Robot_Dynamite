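; BP_DemoPortal is a linked portal that shows a live view from its Destination portal and teleports overlapping, unattached actors there.
; On BeginPlay it spawns a scene capture on the Destination, feeding a render target into the plane's dynamic portal material.
; Tick mirrors the player camera, either rotation only (Simple) or transformed relative to both Outgoing components.
; Teleporting applies the same relative-transform technique and briefly deactivates the Destination to prevent bouncing back.
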(event `self.ReceiveBeginPlay`
  (bind _destination (`self.Destination`))
  (bind _returnvalue (`KismetSystemLibrary.IsValid` (`self.Destination`)))
  (bind _returnvalue_2 (`PrimitiveComponent.CreateDynamicMaterialInstance` (`self.Plane`) 0 "/Game/Robot_Dynamite/Effects/Portal/M_Portal.M_Portal"))
  (bind _returnvalue_3 (`KismetRenderingLibrary.CreateRenderTarget2D` 256))
  (`MaterialInstanceDynamic.SetTextureParameterValue` _returnvalue_2 "RenderTarget" _returnvalue_3)
  (`MaterialInstanceDynamic.SetScalarParameterValue` _returnvalue_2 "Active" (`KismetMathLibrary.Conv_BoolToDouble` _returnvalue))
  (set `self.Active` _returnvalue)
  (`/Engine/EditorBlueprintResources/StandardMacros.IsValid` (`self.Destination`)
    (:`Is Valid`
      (bind _returnvalue_4 (`AddComponent|NODE_AddSceneCaptureComponent2D-0` :`self` _destination :`bManualAttachment` true :`RelativeTransform` (`KismetMathLibrary.MakeTransform` (0.0 0.0 0.0))))
      (bind _output_get (set `self.DestinationSceneCapture` _returnvalue_4))
      (`SceneComponent.K2_AttachToComponent` _returnvalue_4 (`/Game/Robot_Dynamite/Dev/BP_DemoPortal.Outgoing` _destination) "None" "KeepRelative" "KeepRelative" "KeepRelative" true)
      (set `SceneCaptureComponent2D.TextureTarget` _returnvalue_3 _output_get))))

(event `self.Trigger.OnComponentBeginOverlap`
  (params (OverlappedComponent :type "PrimitiveComponent Object Reference") (OtherActor :type "Actor Object Reference") (OtherComp :type "PrimitiveComponent Object Reference") (OtherBodyIndex :type Integer) (bFromSweep :type Boolean) (SweepResult :type "HitResult Structure (by ref)"))
  (`/Engine/EditorBlueprintResources/StandardMacros.IsValid` (`self.GetAttachParentActor` OtherActor)
    (:`Is Not Valid`
      (if (`self.Active`)
        (set `/Game/Robot_Dynamite/Dev/BP_DemoPortal.Active` false (`self.Destination`))
        (`self.K2_SetActorTransform` OtherActor (`/Game/Robot_Dynamite/Base/BPFL_Utilities.AppendTransform` (`self.GetTransform` OtherActor) (`/Game/Robot_Dynamite/Base/BPFL_Utilities.DeltaTransform` (`SceneComponent.K2_GetComponentToWorld` (`/Game/Robot_Dynamite/Dev/BP_DemoPortal.Outgoing` (`self.Destination`))) (`SceneComponent.K2_GetComponentToWorld` (`self.Outgoing`)))) false true)
        (`KismetSystemLibrary.Delay` 0.2)
        (set `/Game/Robot_Dynamite/Dev/BP_DemoPortal.Active` (`KismetSystemLibrary.IsValid` (`/Game/Robot_Dynamite/Dev/BP_DemoPortal.Destination` (`self.Destination`))) (`self.Destination`))))))

(event `self.ReceiveTick`
  (params (DeltaSeconds :type "Float (single-precision)"))
  (bind _destinationscenecapture (`self.DestinationSceneCapture`))
  (bind _transformcomponent (`PlayerCameraManager.TransformComponent` (`GameplayStatics.GetPlayerCameraManager` 0)))
  (bind _returnvalue (`SceneComponent.K2_GetComponentToWorld` (`/Game/Robot_Dynamite/Dev/BP_DemoPortal.Outgoing` (`self.Destination`))))
  (if (`self.Simple`)
    (`SceneComponent.K2_SetWorldRotation` _destinationscenecapture (`SceneComponent.K2_GetComponentRotation` _transformcomponent) false false)
    (else
      (`/Engine/EditorBlueprintResources/StandardMacros.IsValid` (`self.Destination`)
        (:`Is Valid`
          (`SceneComponent.K2_SetWorldTransform` _destinationscenecapture (`/Game/Robot_Dynamite/Base/BPFL_Utilities.AppendTransform` (`SceneComponent.K2_GetComponentToWorld` _transformcomponent) (`/Game/Robot_Dynamite/Base/BPFL_Utilities.DeltaTransform` (`KismetMathLibrary.MakeTransform` (.location _returnvalue) (`KismetMathLibrary.MakeRotator` (.roll (.rotation _returnvalue)) (.pitch (.rotation _returnvalue)) (- 180.0 (.yaw (.rotation _returnvalue)))) (.scale _returnvalue)) (`SceneComponent.K2_GetComponentToWorld` (`self.Outgoing`)))) false false))))))

(fn `UserConstructionScript`)