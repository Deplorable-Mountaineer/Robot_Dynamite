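; Monitor wall actor that displays the live scene capture of a linked BP_Camera, falling back to the first one found.
; On construction and BeginPlay, it points the capture at an assigned or newly created render target and feeds that into a dynamic M_StageRender material.
; Actor X scale follows the aspect ratio relative to 16:9.
; A Snapshot toggle exports the render target as HDR to a hard-coded local path during construction.
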(event `self.ReceiveBeginPlay`
  (`self.Init`))

(fn `AdjustScale`
  (`self.SetActorScale3D` (`KismetMathLibrary.MakeVector` (/ (/ (`KismetMathLibrary.Conv_IntToDouble` (`self.Width`)) 1920.0) (/ (`KismetMathLibrary.Conv_IntToDouble` (`self.Height`)) 1080.0)) 1.0 1.0)))

(fn `Init`
  (`/Engine/EditorBlueprintResources/StandardMacros.IsValid` (`self.Camera`)
    (:`Is Valid`
      (`self.LinkToCamera`)
      (`self.AdjustScale`))
    (:`Is Not Valid`
      (bind _outactors (`GameplayStatics.GetAllActorsOfClass` "/Game/Robot_Dynamite/Dev/BP_Camera.BP_Camera_C"))
      (if (`KismetArrayLibrary.Array_IsValidIndex` _outactors)
        (set `self.Camera` (`|GetArrayItem` _outactors))
        (`self.LinkToCamera`)
        (`self.AdjustScale`)
        (else
          (`PrimitiveComponent.SetMaterial` (`self.SM_MonitorWall`) 1 "/Game/Robot_Dynamite/Dev/M_StageRender.M_StageRender")
          (`self.AdjustScale`))))))

(fn `LinkToCamera`
  (bind _scenecapturecomponent2d (`/Game/Robot_Dynamite/Dev/BP_Camera.SceneCaptureComponent2D` (`self.Camera`)))
  (`/Engine/EditorBlueprintResources/StandardMacros.IsValid` (`self.Render Target`)
    (:`Is Valid`
      (bind _output_get (set `SceneCaptureComponent2D.TextureTarget` (`self.Render Target`) _scenecapturecomponent2d))
      (if (`self.ScaleToRenderTarget`)
        (set `self.Width` (`TextureRenderTarget2D.SizeX` _output_get))
        (set `self.Height` (`TextureRenderTarget2D.SizeY` _output_get))))
    (:`Is Not Valid`
      (bind _returnvalue (`KismetRenderingLibrary.CreateRenderTarget2D` (`self.Width`) (`self.Height`)))
      (bind _output_get_2 (set `SceneCaptureComponent2D.TextureTarget` _returnvalue _scenecapturecomponent2d))
      (bind _output_get_3 (set `self.Render Target` _output_get_2))))
  (bind _returnvalue_2 (`PrimitiveComponent.CreateDynamicMaterialInstance` (`self.SM_MonitorWall`) 1 "/Game/Robot_Dynamite/Dev/M_StageRender.M_StageRender"))
  (`MaterialInstanceDynamic.SetTextureParameterValue` _returnvalue_2 "RenderTarget" _output_get_3))

(fn `UserConstructionScript`
  (`self.Init`)
  (if (`self.Snapshot`)
    (`KismetRenderingLibrary.ExportRenderTarget` (`self.Render Target`) "D:\\Documents\\Repos\\Unreal4\\Robot_Dynamite\\Content\\Robot_Dynamite\\Dev" "BP_Monitor_Snapshot.hdr")
    (set `self.Snapshot` false)))