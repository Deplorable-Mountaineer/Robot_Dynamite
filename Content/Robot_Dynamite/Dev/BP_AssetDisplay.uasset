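; BP_AssetDisplay is a development display actor in the Robot_Dynamite folder that shows one chosen asset with its name as a text label.
; The construction script takes the first valid input in priority order: skeletal mesh, static mesh, then actor class.
; It assigns that input to the matching mesh or child actor component and sets the text render to its display name.
; The event graph has no active logic.
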(fn `UserConstructionScript`
  (bind _usestaticmesh (`self.UseStaticMesh`))
  (bind _useskeletalmesh (`self.UseSkeletalMesh`))
  (bind _useactor (`self.UseActor`))
  (`/Engine/EditorBlueprintResources/StandardMacros.IsValid` _useskeletalmesh
    (:`Is Valid`
      (`SkinnedMeshComponent.SetSkinnedAssetAndUpdate` (`self.SkeletalMesh`) _useskeletalmesh true)
      (`TextRenderComponent.K2_SetText` (`self.TextRender`) (`KismetTextLibrary.Conv_StringToText` (`KismetSystemLibrary.GetDisplayName` _useskeletalmesh))))
    (:`Is Not Valid`
      (`/Engine/EditorBlueprintResources/StandardMacros.IsValid` _usestaticmesh
        (:`Is Valid`
          (`StaticMeshComponent.SetStaticMesh` (`self.StaticMesh`) _usestaticmesh)
          (`TextRenderComponent.K2_SetText` (`self.TextRender`) (`KismetTextLibrary.Conv_StringToText` (`KismetSystemLibrary.GetDisplayName` _usestaticmesh))))
        (:`Is Not Valid`
          (if (`KismetSystemLibrary.IsValidClass` _useactor)
            (`ChildActorComponent.SetChildActorClass` (`self.ChildActor`) _useactor)
            (`TextRenderComponent.K2_SetText` (`self.TextRender`) (`KismetTextLibrary.Conv_StringToText` (`KismetSystemLibrary.GetClassDisplayName` _useactor)))))))))