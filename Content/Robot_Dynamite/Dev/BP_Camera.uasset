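; BP_Camera is an actor that aims itself at a target location when its construction script runs.
; It uses the assigned LightTarget, or falls back to the first TargetPoint found in the level.
; FaceTarget rotates the actor's X axis toward that target, or toward the stored LightTargetLocation when no target exists.
; The event graph is empty, so it does not track the target during play.
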(fn `Face Target`
  (if (`self.bUse Light Target Actor`)
    (set `self.Light Target Location` (`self.K2_GetActorLocation` (`self.Light Target`))))
  (`self.K2_SetActorRotation` (`KismetMathLibrary.Conv_VectorToRotator` (- (`self.Light Target Location`) (`self.K2_GetActorLocation`)))))

(fn `UserConstructionScript`
  (`/Engine/EditorBlueprintResources/StandardMacros.IsValid` (`self.Light Target`)
    (:`Is Valid`
      (set `self.bUse Light Target Actor` true)
      (`self.Face Target`))
    (:`Is Not Valid`
      (bind _outactors (`GameplayStatics.GetAllActorsOfClass` "/Script/Engine.TargetPoint"))
      (if (`KismetArrayLibrary.Array_IsValidIndex` _outactors)
        (set `self.Light Target` (`|GetArrayItem` _outactors))
        (set `self.bUse Light Target Actor` true)
        (`self.Face Target`)
        (else
          (set `self.bUse Light Target Actor` false)
          (`self.Face Target`))))))