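; BP_Inventory_C is a character inventory that stores items in an array keyed by each item's own Index.
; Add writes the item into that slot, growing the array as needed, then calls its Stash and OnPickUp.
; Has checks a slot for a valid item and returns it with its inner Item.
; Discard removes and returns the entry, which shifts later items down from their assigned slots.
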(fn `Add`
  (params (InventoryItem :type "/Game/Robot_Dynamite/Characters/BP_InventoryItem Object Reference"))
  (`KismetArrayLibrary.Array_Set` (`self.Items`) (`/Game/Robot_Dynamite/Characters/BP_InventoryItem.Index` InventoryItem) InventoryItem true)
  (`/Game/Robot_Dynamite/Characters/BP_InventoryItem.Stash` InventoryItem)
  (`/Game/Robot_Dynamite/Characters/BP_InventoryItem.OnPickUp` InventoryItem)
  (return))

(fn `Discard`
  (params (Index :type Integer))
  (returns (InventoryItem :type "/Game/Robot_Dynamite/Characters/BP_InventoryItem Object Reference"))
  (locals (TempItem :type "/Game/Robot_Dynamite/Characters/BP_InventoryItem Object Reference"))
  (bind _items (`self.Items`))
  (bind _output_get (set `local.TempItem` (`|GetArrayItem` _items Index)))
  (`KismetArrayLibrary.Array_Remove` _items Index)
  (return _output_get))

(fn `Has`
  (params (Index :type Integer))
  (returns (InventoryItem :type "/Game/Robot_Dynamite/Characters/BP_InventoryItem Object Reference") (ActualItem :type "Actor Object Reference") (True :type Boolean))
  (bind _output (`|GetArrayItem` (`self.Items`) Index))
  (if (`KismetArrayLibrary.Array_IsValidIndex` (`self.Items`) Index)
    (return _output (`/Game/Robot_Dynamite/Characters/BP_InventoryItem.Item` _output) (`KismetSystemLibrary.IsValid` _output))
    (else
      (return null null false))))