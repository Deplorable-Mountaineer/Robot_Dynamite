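; BP_Inventory is an inventory actor that sets up a character's fixed set of weapon and pickup slots at BeginPlay.
; CreateInventorySlot spawns a BP_InventorySlot holding item class, messages, icon and usage flags, then stores it at an explicit index in the Slots array.
; Melee, health and armor items spawn immediately, while rifle and grenade launcher slots start without an item.
; Spawned actors are owned by the parent actor, with weapons and stats in separate index ranges.
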(event EventBeginPlay
  (CallFunction|CreateInventorySlot 0 "/Game/Robot_Dynamite/Weapons/Melee/BP_Melee.BP_Melee_C" 0 "" "" "" "/Game/Robot_Dynamite/Characters/Player/T_PlayerLogo_D.T_PlayerLogo_D" false false true)
  (CallFunction|CreateInventorySlot 1 "/Game/Robot_Dynamite/Weapons/Rifle/BP_Rifle.BP_Rifle_C" 0 "Got Rifle" "Using Rifle" "Reloaded Rifle" "/Game/Robot_Dynamite/Characters/Player/T_PlayerLogo_D.T_PlayerLogo_D" false true false)
  (CallFunction|CreateInventorySlot 2 "/Game/Robot_Dynamite/Weapons/GrenadeLauncher/BP_GrenadeLauncher.BP_GrenadeLauncher_C" 0 "Got Grenade Launcher" "Using Grenade Launcher" "Reloaded Grenade Launcher" "/Game/Robot_Dynamite/Characters/Player/T_PlayerLogo_D.T_PlayerLogo_D" false true false)
  (CallFunction|CreateInventorySlot 20 "/Game/Robot_Dynamite/Characters/BP_Health.BP_Health_C" 0 "" "" "Replenished Health" "/Game/Robot_Dynamite/Characters/Player/T_PlayerLogo_D.T_PlayerLogo_D" false true true)
  (CallFunction|CreateInventorySlot 21 "/Game/Robot_Dynamite/Characters/BP_Armor.BP_Armor_C" 0 "" "" "Replenished Armor" "/Game/Robot_Dynamite/Characters/Player/T_PlayerLogo_D.T_PlayerLogo_D" false true true))

(fn ConstructionScript)

(fn CreateInventorySlot
  (params (Index :type Integer) (ItemClass :type Actor%20Class%20Reference) (Item :type Actor%20Object%20Reference) (TextOnPickup :type String) (TextOnUse :type String) (TextOnReload :type String) (Image :type Texture%20Object%20Reference) (DiscardOnUse :type Boolean) (Reloadable :type Boolean) (SpawnTheItem :type Boolean))
  (bind _returnvalue (Math|Transform|MakeTransform "0, 0, 0"))
  (bind _returnvalue_2 (Actor|GetParentActor))
  (if SpawnTheItem
    (bind _returnvalue_3 (Game|SpawnActorfromClass ItemClass _returnvalue "AdjustIfPossibleButAlwaysSpawn" _returnvalue_2 (stale _aspawn))))
  (bind _returnvalue_4 (Game|SpawnActorfromClass "/Game/Robot_Dynamite/Characters/BP_InventorySlot.BP_InventorySlot_C" _returnvalue "AlwaysSpawn" _returnvalue_2 ItemClass (select SpawnTheItem _returnvalue_3 Item) TextOnPickup TextOnUse TextOnReload Image DiscardOnUse Reloadable (stale _aspawn)))
  (Utilities|Array|SetArrayElem (Variables|Default|GetSlots) Index _returnvalue_4 true)
  (return))