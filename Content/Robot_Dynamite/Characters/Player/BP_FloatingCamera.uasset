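; BP_FloatingCamera is a player camera actor that drifts upward and backward through the scene.
; Each Tick it offsets its location along its own up vector by RiseSpeed and against its forward vector by BackSpeed, both scaled by delta time.
; The move uses no sweep, so it ignores collision, and it never changes rotation.
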(event `self.ReceiveTick`
  (params (DeltaSeconds :type "Float (single-precision)"))
  (`self.K2_SetActorLocation` (- (+ (* (* (`self.GetActorUpVector`) DeltaSeconds) (`self.RiseSpeed`)) (`self.K2_GetActorLocation`)) (* (* (`self.GetActorForwardVector`) DeltaSeconds) (`self.BackSpeed`)))))

(fn `UserConstructionScript`)