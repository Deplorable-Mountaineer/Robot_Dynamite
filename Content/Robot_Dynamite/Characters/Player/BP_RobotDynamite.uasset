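; Player character Blueprint for Robot Dynamite, extending a parent's inventory, death and HUD events with first-person firing animation and weapon attachment.
; BeginPlay spawns a BP_Messages actor and creates the HUD widget.
; OnHUDUpdate copies four message lines, health, armor, ammo and power-up status into display variables after a short delay.
; Toggleable night vision overwrites settings on PostProcess volumes tagged "NightVision", with a delayed Tick check for power-up depletion.
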(event `/Game/Robot_Dynamite/Base/BPI_Character.GunFired`
  ;[1 0.198 0] Fire Animation
  (`AnimInstance.Montage_Play` (`SkeletalMeshComponent.GetAnimInstance` (`self.ArmsFP`)) "/Game/Robot_Dynamite/Characters/Player/AM_FireFP.AM_FireFP" 1.0 "MontageLength" 0.0))

(event `self.OnDeath`
  ;[1 1 1] Death
  (`self.Player_Die`))

(event `self.ReceiveBeginPlay`
  ;[1 1 1] Startup
  (`parent.ReceiveBeginPlay`)
  (bind _returnvalue (`|SpawnActorFromClass` "/Game/Robot_Dynamite/UI/BP_Messages.BP_Messages_C" (`KismetMathLibrary.MakeTransform` (0.0 0.0 0.0)) "AlwaysSpawn" "OverrideRootScale" self self))
  (set `self.Messages` _returnvalue)
  (bind _returnvalue_2 (`|CreateWidget` "/Game/Robot_Dynamite/UI/BP_HUD_Widget.BP_HUD_Widget_C" (`GameplayStatics.GetPlayerController` 0)))
  (`UserWidget.AddToViewport` _returnvalue_2 0)
  (set `self.HUD Widget` _returnvalue_2))

(event `self.On Inventory Spawn`
  (params (Item :type "/Game/Robot_Dynamite/Inventory/BP_Item Object Reference") (Socket :type Name))
  (`parent.On Inventory Spawn` Item Socket)
  (bind _asbp_weapon (cast `/Game/Robot_Dynamite/Inventory/BP_Weapon` Item))
  (`self.K2_AttachToComponent` _asbp_weapon (`self.ArmsFP`) Socket "KeepRelative" "KeepRelative" "KeepRelative" true)
  (bind _sk_gun (`/Game/Robot_Dynamite/Inventory/BP_Weapon.SK_Gun` _asbp_weapon))
  (`SkinnedMeshComponent.SetSkinnedAssetAndUpdate` (`self.TPGun`) (`SkinnedMeshComponent.SkeletalMesh` _sk_gun) true)
  (`SceneComponent.SetVisibility` _sk_gun (`SceneComponent.IsVisible` (`Actor.RootComponent` Item)) false))

(event `self.OnWeaponSelect`
  (params (Weapon :type "/Game/Robot_Dynamite/Inventory/BP_Weapon Object Reference") (Socket :type Name))
  ;[1 1 1] On Weapon Select
  (`parent.OnWeaponSelect` Weapon Socket))

(event `InputAction|Use Night Vision`
  (params (Key :type "Key Structure"))
  ;[1 1 1] Night Vision
  (:`Pressed`
    (`self.NVG`)))

(event `NVG`
  (`/Engine/EditorBlueprintResources/StandardMacros.FlipFlop`
    (:`A`
      (bind _success (`self.SelectInventory` "/Game/Robot_Dynamite/Inventory/PowerUps/BP_NVG.BP_NVG_C"))
      (if _success
        (`self.Start Night Vision`)
        (else
          (`self.NVG`))))
    (:`B`
      (`self.Stop Night Vision`)
      (set `self.CurrentPowerUp` null))))

(event `self.Does Not Have`
  (params (What :type String))
  (`/Game/Robot_Dynamite/Base/BPML_Utilities_Actors.DisplayMessage` (`KismetStringLibrary.Concat_StrStr` "Robot Dynamite does not have powerup: " What)))

(event `self.ReceiveTick`
  (params (DeltaSeconds :type "Float (single-precision)"))
  (`parent.ReceiveTick` DeltaSeconds)
  (`KismetSystemLibrary.Delay` 1.021)
  (bind _depleted (`self.UseUpNVG`))
  (if _depleted
    (`self.NVG`)))

(event `self.On HUD Update`
  (bind _textcolor (`/Game/Robot_Dynamite/UI/BP_Messages.TextColor` (`self.Messages`)))
  (bind _text (`/Game/Robot_Dynamite/UI/BP_Messages.Text` (`self.Messages`)))
  (`parent.On HUD Update`)
  (`KismetSystemLibrary.Delay` 0.1)
  ;[1 1 1] Comment
  (`|ExecutionSequence`
    (:`then_0`
      (set `self.MessageLine1` (`KismetTextLibrary.Conv_StringToText` (`|GetArrayItem` _text)))
      (set `self.MessageColor1` (`|GetArrayItem` _textcolor)))
    (:`then_1`
      (set `self.MessageLine2` (`KismetTextLibrary.Conv_StringToText` (`|GetArrayItem` _text 1)))
      (set `self.MessageColor2` (`|GetArrayItem` _textcolor 1)))
    (:`then_2`
      (set `self.MessageLine3` (`KismetTextLibrary.Conv_StringToText` (`|GetArrayItem` _text 2)))
      (set `self.MessageColor3` (`|GetArrayItem` _textcolor 2)))
    (:`then_3`
      (set `self.MessageLine4` (`KismetTextLibrary.Conv_StringToText` (`|GetArrayItem` _text 3)))
      (set `self.MessageColor4` (`|GetArrayItem` _textcolor 3)))
    (:`then_4`
      (`|ExecutionSequence`
        (:`then_0`
          (bind _amount (`self.GetVitalStatistic` "/Game/Robot_Dynamite/Inventory/VitalStatistics/BP_Health.BP_Health_C"))
          (set `self.Health` (`KismetTextLibrary.Conv_DoubleToText` _amount "ToPositiveInfinity" true 1 324 0 0)))
        (:`then_1`
          (bind _amount_2 (`self.GetVitalStatistic` "/Game/Robot_Dynamite/Inventory/VitalStatistics/BP_Armor.BP_Armor_C"))
          (set `self.Armor` (`KismetTextLibrary.Conv_DoubleToText` _amount_2 "ToPositiveInfinity" true 1 324 0 0)))
        (:`then_2`
          (bind _ammoamount (`self.GetCurrentAmmo`))
          (set `self.Ammo` (`KismetTextLibrary.Conv_DoubleToText` _ammoamount "ToPositiveInfinity" true 1 324 0 0))
          (set `self.AmmoName` (`KismetTextLibrary.Conv_StringToText` (`/Game/Robot_Dynamite/Inventory/BP_Item.Item Name` (`self.CurrentGun`)))))
        (:`then_3`
          (bind (_ammoamount_2 _isvalid) (`self.GetCurrentPowerUp`))
          (if _isvalid
            (set `self.Inv` (`KismetTextLibrary.Conv_DoubleToText` _ammoamount_2 "ToPositiveInfinity" true 1 324 0 0))
            (set `self.InvName` (`KismetTextLibrary.Conv_StringToText` (`/Game/Robot_Dynamite/Inventory/BP_Item.Item Name` (`self.CurrentPowerUp`))))
            (else
              (set `self.Inv` "")
              (set `self.InvName` "Power Up"))))))))

(fn `DisplayMessage`
  (params (Text :type String) (TextColor :type "LinearColor Structure" :default (struct :`G` 1.0 :`B` 0.5 :`A` 1.0)))
  (bind _messages (`self.Messages`))
  (`/Engine/EditorBlueprintResources/StandardMacros.IsValid` _messages
    (:`Is Valid`
      (`/Game/Robot_Dynamite/UI/BP_Messages.NewMessage` _messages Text TextColor)
      (return))
    (:`Is Not Valid`
      (`KismetSystemLibrary.PrintString` Text true true TextColor))))

(fn `Start Night Vision`
  (if (not (`self.bNVG`))
    (bind _outactors (`GameplayStatics.GetAllActorsWithTag` "NightVision"))
    (if (<= (`KismetArrayLibrary.Array_Length` _outactors) 0)
      (`/Game/Robot_Dynamite/Base/BPML_Utilities_Actors.Error` "No PostProcess Volumes tagged \"NightVision\" found in level!")
      (return)
      (else
        (for _array_element _outactors
          (bind _aspost_process_volume (cast `PostProcessVolume` _array_element)
            (:`then`
              (set `PostProcessVolume.Settings` (make `PostProcessSettings` :`SceneColorTint` (struct :`G` 1.0 :`B` 0.5 :`A` 1.0) :`SceneFringeIntensity` 5.0 :`AmbientCubemap` "/Game/Robot_Dynamite/Effects/Lighting/NightVision.NightVision" :`VignetteIntensity` 1.0 :`GrainJitter` 1.0 :`GrainIntensity` 1.0) _aspost_process_volume)
              (set `self.bNVG` true)
              (return))
            (:`CastFailed`
              (`/Game/Robot_Dynamite/Base/BPML_Utilities_Actors.Error` "Actor tagged \"NightVision\" is not a postprocess volume: " (`KismetSystemLibrary.GetDisplayName` _array_element))
              (return))))))))

(fn `Stop Night Vision`
  (if (`self.bNVG`)
    (bind _outactors (`GameplayStatics.GetAllActorsWithTag` "NightVision"))
    (for _array_element _outactors
      (bind _aspost_process_volume (cast `PostProcessVolume` _array_element))
      (set `PostProcessVolume.Settings` (make `PostProcessSettings` :`AmbientCubemapIntensity` 0.0 :`VignetteIntensity` 0.0) _aspost_process_volume)
      (set `self.bNVG` false))))

(fn `UserConstructionScript`
  (`parent.UserConstructionScript`))