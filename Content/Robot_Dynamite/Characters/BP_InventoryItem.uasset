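; BP_InventoryItem represents one inventory entry for a BP_Character, wrapping a spawned item actor with its display and configuration data.
; On BeginPlay, Init spawns ItemClass with the instigator as owner and attaches it to a configured component socket.
; OnUse shows the item, Stash hides it, and Reconfigure overwrites the entry's settings.
; Pickup, use and reload events display colored messages, printing on screen only for the player, with reload gated by ReloadMessage.
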(event `self.ReceiveBeginPlay`
  (`self.Init`))

(event `OnPickUp`
  (bind _returnvalue (`self.GetInstigator`))
  (bind _asbp_character (cast `/Game/Robot_Dynamite/Characters/BP_Character` _returnvalue))
  (`/Game/Robot_Dynamite/Base/BPFL_Utilities.DisplayMessage` (`self.TextOnPickup`) (and (`/Game/Robot_Dynamite/Characters/BP_Character.bPlayer` _asbp_character) (`Pawn.IsPlayerControlled` _returnvalue)) true (`self.OnPickupTextColor`)))

(event `OnUse`
  (bind _returnvalue (`self.GetInstigator`))
  (bind _asbp_character (cast `/Game/Robot_Dynamite/Characters/BP_Character` _returnvalue))
  (`/Game/Robot_Dynamite/Base/BPFL_Utilities.DisplayMessage` (`self.TextOnUse`) (and (`/Game/Robot_Dynamite/Characters/BP_Character.bPlayer` _asbp_character) (`Pawn.IsPlayerControlled` _returnvalue)) true (`self.OnUseTextColor`))
  (`SceneComponent.SetVisibility` (`self.K2_GetRootComponent` (`self.Item`)) true true))

(event `OnReload`
  (params (Amount :type Integer) (IgnoreMax :type Boolean))
  (bind _returnvalue (`self.GetInstigator`))
  (bind _bamountchanged (message `/Game/Robot_Dynamite/Base/BPI_Reloadable.Reload` (`self.Item`) 0.0 IgnoreMax))
  (if _bamountchanged
    (bind _asbp_character (cast `/Game/Robot_Dynamite/Characters/BP_Character` _returnvalue))
    (`/Game/Robot_Dynamite/Base/BPFL_Utilities.DisplayMessage` (`self.TextOnReload`) (and (`/Game/Robot_Dynamite/Characters/BP_Character.bPlayer` _asbp_character) (`Pawn.IsPlayerControlled` _returnvalue)) true (`self.OnReloadTextColor`))))

(fn `Init`
  (bind _returnvalue (`self.GetInstigator`))
  (bind _returnvalue_2 (`|SpawnActorFromClass` (`self.ItemClass`) (`KismetMathLibrary.MakeTransform` (0.0 0.0 0.0)) "AlwaysSpawn" "OverrideRootScale" _returnvalue _returnvalue))
  (bind _output_get (set `self.Item` _returnvalue_2))
  (`self.K2_AttachToComponent` _output_get (`self.AttachParentComponent`) (`self.AttachSocketName`) "KeepRelative" "KeepRelative" "KeepRelative" true))

(fn `Reconfigure`
  (params (Index :type Integer :default -1) (ItemClass :type "Actor Class Reference") (AttachParentComponent :type "SceneComponent Object Reference") (AttachSocketName :type Name :default "GripPoint") (Name :type Name :default "Inventory Item") (TextOnPickup :type String :default "Got Inventory Item") (TextOnUse :type String :default "Using Inventory Item") (TextOnReload :type String :default "Reloaded Inventory Item") (OnPickupTextColor :type "LinearColor Structure" :default (struct :`G` 0.66 :`B` 1.0 :`A` 1.0)) (OnUseTextColor :type "LinearColor Structure" :default (struct :`R` 0.66 :`G` 1.0 :`A` 1.0)) (OnReloadTextColor :type "LinearColor Structure" :default (struct :`R` 1.0 :`G` 0.66 :`A` 1.0)) (Image :type "Texture Object Reference") (bDiscardOnUse :type Boolean) (bSuper :type Boolean))
  (set `self.Index` Index)
  (set `self.ItemClass` ItemClass)
  (`/Engine/EditorBlueprintResources/StandardMacros.IsValid` AttachParentComponent
    (:`Is Valid`
      (set `self.AttachParentComponent` AttachParentComponent))
    (:`Is Not Valid`
      _))
  (set `self.AttachSocketName` AttachSocketName)
  (set `self.Name` Name)
  (set `self.TextOnPickup` TextOnPickup)
  (set `self.TextOnUse` TextOnUse)
  (set `self.TextOnReload` TextOnReload)
  (set `self.OnPickupTextColor` OnPickupTextColor)
  (set `self.OnUseTextColor` OnUseTextColor)
  (set `self.OnReloadTextColor` OnReloadTextColor)
  (`/Engine/EditorBlueprintResources/StandardMacros.IsValid` Image
    (:`Is Valid`
      (set `self.Image` Image))
    (:`Is Not Valid`
      _))
  (set `self.bDiscardOnUse` bDiscardOnUse)
  (set `self.bSuper` bSuper))

(fn `Stash`
  (`SceneComponent.SetVisibility` (`self.K2_GetRootComponent` (`self.Item`)) false true)
  (return))

(fn `UserConstructionScript`)