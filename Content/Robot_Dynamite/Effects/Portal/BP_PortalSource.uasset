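; Source end of a linked portal pair that shows the other side's view and teleports overlapping actors to its destination.
; Construction cross-links both portals' scene captures and render targets, displaying the result through a dynamic M_Portal material.
; BeginPlay precomputes forward and return transform deltas, and trigger overlaps apply the forward one.
; Pawns are unpossessed and repossessed around the move, with the destination briefly disabled; Retarget relinks at runtime.
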(event `self.ReceiveBeginPlay`
  (`self.SetupAtConstruction`)
  (`self.SetupAtBeginPlay`))

(event `self.Triger.OnComponentBeginOverlap`
  (params (OverlappedComponent :type "PrimitiveComponent Object Reference") (OtherActor :type "Actor Object Reference") (OtherComp :type "PrimitiveComponent Object Reference") (OtherBodyIndex :type Integer) (bFromSweep :type Boolean) (SweepResult :type "HitResult Structure (by ref)"))
  (bind _rootcomponent (`Actor.RootComponent` OtherActor))
  (bind _result (`self.AddDelta` (`SceneComponent.K2_GetComponentToWorld` _rootcomponent) (`self.Delta`)))
  (if (not (`self.bDisable`))
    (bind _aspawn (cast `Pawn` OtherActor)
      (:`then`
        (set `/Game/Robot_Dynamite/Effects/Portal/BP_PortalDest.bDisable` true (`self.Dest`))
        (bind _output_get (set `self.PawnController` (`Pawn.GetController` _aspawn)))
        (`Pawn.DetachFromControllerPendingDestroy` _aspawn)
        (`SceneComponent.K2_SetWorldTransform` _rootcomponent _result false true)
        (`Controller.Possess` _output_get _aspawn)
        (set `/Game/Robot_Dynamite/Effects/Portal/BP_PortalDest.bDisable` false (`self.Dest`)))
      (:`CastFailed`
        (`SceneComponent.K2_SetWorldTransform` _rootcomponent _result false true)))))

(fn `AddDelta`
  (params (Initial :type "Transform Structure") (Addend :type "Transform Structure"))
  (returns (Result :type "Transform Structure"))
  (return (`KismetMathLibrary.MakeTransform` (+ Initial_Location Addend_Location) (`KismetMathLibrary.ComposeRotators` Initial_Rotation Addend_Rotation) (`KismetMathLibrary.MakeVector` (* (.x (.scale Initial)) (.x (.scale Addend))) (* (.y (.scale Initial)) (.y (.scale Addend))) (* (.z (.scale Initial)) (.z (.scale Addend)))))))

(fn `DeltaTransform`
  (params (Dest :type "Transform Structure") (Source :type "Transform Structure"))
  (returns (Delta :type "Transform Structure"))
  (return (`KismetMathLibrary.MakeTransform` (- Dest_Location Source_Location) (`KismetMathLibrary.NormalizedDeltaRotator` Dest_Rotation Source_Rotation) (`KismetMathLibrary.MakeVector` (/ (.x (.scale Dest)) (.x (.scale Source))) (/ (.y (.scale Dest)) (.y (.scale Source))) (/ (.z (.scale Dest)) (.z (.scale Source)))))))

(fn `Retarget`
  (params (NewDest :type "/Game/Robot_Dynamite/Effects/Portal/BP_PortalDest Object Reference"))
  (set `self.Dest` NewDest)
  (`self.SetupAtConstruction`)
  (`self.SetupAtBeginPlay`))

(fn `SetupAtBeginPlay`
  (set `self.Delta` (`self.DeltaTransform` (`SceneComponent.K2_GetComponentToWorld` (`|GetArrayItem` (`self.GetComponentsByTag` (`self.Dest`) "/Script/Engine.ArrowComponent" "MaterializeTarget"))) (`SceneComponent.K2_GetComponentToWorld` (`self.Triger`))))
  (set `self.ReturnDelta` (`self.DeltaTransform` (`SceneComponent.K2_GetComponentToWorld` (`self.MaterializeHere`)) (`SceneComponent.K2_GetComponentToWorld` (`|GetArrayItem` (`self.GetComponentsByTag` (`self.Dest`) "/Script/Engine.BoxComponent" "Trigger"))))))

(fn `SetupAtConstruction`
  (bind _dest (`self.Dest`))
  (bind _returnvalue (`KismetRenderingLibrary.CreateRenderTarget2D` 512 512))
  (set `self.RenderTarget` _returnvalue)
  (bind _returnvalue_2 (`KismetMaterialLibrary.CreateDynamicMaterialInstance` "/Game/Robot_Dynamite/Effects/Portal/M_Portal.M_Portal"))
  (`PrimitiveComponent.SetMaterial` (`self.Plane`) 0 _returnvalue_2)
  (`MaterialInstanceDynamic.SetTextureParameterValue` _returnvalue_2 "RenderTarget" _returnvalue)
  (`/Engine/EditorBlueprintResources/StandardMacros.IsValid` _dest
    (:`Is Valid`
      (`/Game/Robot_Dynamite/Effects/Portal/BP_PortalDest.Setup` _dest)
      (set `SceneCaptureComponent2D.TextureTarget` (`self.RenderTarget`) (`/Game/Robot_Dynamite/Effects/Portal/BP_PortalDest.SceneCaptureComponent2D` _dest))
      (set `SceneCaptureComponent2D.TextureTarget` (`/Game/Robot_Dynamite/Effects/Portal/BP_PortalDest.RenderTarget` _dest) (`self.SceneCaptureComponent2D`))
      (set `/Game/Robot_Dynamite/Effects/Portal/BP_PortalDest.Source` self _dest))))

(fn `UserConstructionScript`
  (`self.SetupAtConstruction`))