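; BP_DynamicWaterZone is a water zone that makes overlapping BP_Character actors swim and can apply environmental damage.
; Volume overlaps toggle Swimming or Walking and set the WaterVolume flag on the character's current physics volume.
; RequireInWater selects whether PainVolume or Volume sets the character's EnvironmentalDamage to DamagePerSecond on entry and zero on exit.
; The construction script is empty, with a disconnected "Water Height" parameter setter.
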(event `self.Volume.OnComponentBeginOverlap`
  (params (OverlappedComponent :type "PrimitiveComponent Object Reference") (OtherActor :type "Actor Object Reference") (OtherComp :type "PrimitiveComponent Object Reference") (OtherBodyIndex :type Integer) (bFromSweep :type Boolean) (SweepResult :type "HitResult Structure (by ref)"))
  ;[1 1 1] Under Water
  (bind _asbp_character (cast `/Game/Robot_Dynamite/Characters/BP_Character` OtherActor))
  (bind _charactermovement (`Character.CharacterMovement` _asbp_character))
  (`CharacterMovementComponent.SetMovementMode` _charactermovement "MOVE_Swimming" 0)
  (set `PhysicsVolume.bWaterVolume` true (`MovementComponent.GetPhysicsVolume` _charactermovement))
  (if (not (`self.bRequireInWater`))
    (set `/Game/Robot_Dynamite/Characters/BP_Character.EnvironmentalDamage` (`self.DamagePerSecond`) _asbp_character)))

(event `self.Volume.OnComponentEndOverlap`
  (params (OverlappedComponent :type "PrimitiveComponent Object Reference") (OtherActor :type "Actor Object Reference") (OtherComp :type "PrimitiveComponent Object Reference") (OtherBodyIndex :type Integer))
  ;[1 1 1] Under Water
  (bind _asbp_character (cast `/Game/Robot_Dynamite/Characters/BP_Character` OtherActor))
  (bind _charactermovement (`Character.CharacterMovement` _asbp_character))
  (`CharacterMovementComponent.SetMovementMode` _charactermovement "MOVE_Walking" 0)
  (set `PhysicsVolume.bWaterVolume` false (`MovementComponent.GetPhysicsVolume` _charactermovement))
  (if (not (`self.bRequireInWater`))
    (set `/Game/Robot_Dynamite/Characters/BP_Character.EnvironmentalDamage` 0.0 _asbp_character)))

(event `self.PainVolume.OnComponentBeginOverlap`
  (params (OverlappedComponent :type "PrimitiveComponent Object Reference") (OtherActor :type "Actor Object Reference") (OtherComp :type "PrimitiveComponent Object Reference") (OtherBodyIndex :type Integer) (bFromSweep :type Boolean) (SweepResult :type "HitResult Structure (by ref)"))
  (bind _asbp_character (cast `/Game/Robot_Dynamite/Characters/BP_Character` OtherActor))
  (if (`self.bRequireInWater`)
    (set `/Game/Robot_Dynamite/Characters/BP_Character.EnvironmentalDamage` (`self.DamagePerSecond`) _asbp_character)))

(event `self.PainVolume.OnComponentEndOverlap`
  (params (OverlappedComponent :type "PrimitiveComponent Object Reference") (OtherActor :type "Actor Object Reference") (OtherComp :type "PrimitiveComponent Object Reference") (OtherBodyIndex :type Integer))
  (bind _asbp_character (cast `/Game/Robot_Dynamite/Characters/BP_Character` OtherActor))
  (if (`self.bRequireInWater`)
    (set `/Game/Robot_Dynamite/Characters/BP_Character.EnvironmentalDamage` 0.0 _asbp_character)))

(fn `UserConstructionScript`)