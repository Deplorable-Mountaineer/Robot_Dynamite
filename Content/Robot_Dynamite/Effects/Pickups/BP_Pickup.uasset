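; BP_Pickup is a world pickup that gives its child-actor inventory item to any BP_Character overlapping its collider.
; It initializes the item on BeginPlay, then on overlap either adds it to the inventory or, when ReloadOnly is set, reloads a matching reloadable by the item's amount.
; It destroys itself only when that transfer succeeds, and its Destroyed event plays the pickup sound at its location.
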(event `self.ReceiveBeginPlay`
  (bind _asbp_inventory_item (cast `/Game/Robot_Dynamite/Characters/BP_InventoryItem` (`ChildActorComponent.ChildActor` (`self.Inventory Item`))))
  (`/Game/Robot_Dynamite/Characters/BP_InventoryItem.Init` _asbp_inventory_item))

(event `self.Collider.OnComponentBeginOverlap`
  (params (OverlappedComponent :type "PrimitiveComponent Object Reference") (OtherActor :type "Actor Object Reference") (OtherComp :type "PrimitiveComponent Object Reference") (OtherBodyIndex :type Integer) (bFromSweep :type Boolean) (SweepResult :type "HitResult Structure (by ref)"))
  (if (`self.bReloadOnly`)
    (bind _asbp_character (cast `/Game/Robot_Dynamite/Characters/BP_Character` OtherActor))
    (bind _asbp_inventory_item (cast `/Game/Robot_Dynamite/Characters/BP_InventoryItem` (`ChildActorComponent.ChildActor` (`self.Inventory Item`))))
    (bind _amount (message `/Game/Robot_Dynamite/Base/BPI_Reloadable.GetAmount` (`/Game/Robot_Dynamite/Characters/BP_InventoryItem.Item` _asbp_inventory_item)))
    (bind (_inventoryitem _actualitem _success) (`/Game/Robot_Dynamite/Characters/BP_Character.ReloadReloadableInInventory` _asbp_character (`/Game/Robot_Dynamite/Characters/BP_InventoryItem.Index` _asbp_inventory_item) _amount (`/Game/Robot_Dynamite/Characters/BP_InventoryItem.bSuper` _asbp_inventory_item)))
    (if _success
      (`self.K2_DestroyActor`))
    (else
      (bind _asbp_character_2 (cast `/Game/Robot_Dynamite/Characters/BP_Character` OtherActor))
      (bind _asbp_inventory_item_2 (cast `/Game/Robot_Dynamite/Characters/BP_InventoryItem` (`ChildActorComponent.ChildActor` (`self.Inventory Item`))))
      (bind _success_2 (`/Game/Robot_Dynamite/Characters/BP_Character.AddToInventory` _asbp_character_2 _asbp_inventory_item_2))
      (if _success_2
        (`self.K2_DestroyActor`)))))

(event `self.ReceiveDestroyed`
  (`GameplayStatics.PlaySoundAtLocation` (`self.PickupSound`) (`SceneComponent.K2_GetComponentLocation` (`self.DefaultSceneRoot`))))

(fn `UserConstructionScript`)