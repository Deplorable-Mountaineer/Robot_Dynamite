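; BP_LCD_Component drives an LCD text display on a mesh material slot.
; On Init, it creates a dynamic MI_LCD instance and binds a BP_LCD canvas render target as its texture, then shows default orange "Robot Dynamite" text.
; SetRenderTextureParameters passes text, color and scale to the render target, mirrors scale to the material, and updates the resource to redraw.
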(event `Init`
  (bind _returnvalue (`PrimitiveComponent.CreateDynamicMaterialInstance` (`self.LCD Mesh Component`) (`self.LCD Material Index`) "/Game/Robot_Dynamite/Effects/LCD/MI_LCD.MI_LCD"))
  (set `self.Material` _returnvalue)
  (bind _returnvalue_2 (`CanvasRenderTarget2D.CreateCanvasRenderTarget2D` "/Game/Robot_Dynamite/Effects/LCD/BP_LCD.BP_LCD_C" 256 256))
  (bind _output_get (set `self.RenderTexture` (cast `/Game/Robot_Dynamite/Effects/LCD/BP_LCD` _returnvalue_2 :!pure true)))
  (`MaterialInstanceDynamic.SetTextureParameterValue` (`self.Material`) "Target Texture" _output_get)
  (`self.SetRenderTextureParameters` "Robot \nDynamite"))

(fn `SetRenderTextureParameters`
  (params (Text :type Text :default "Robot \nDynamite") (Color :type "LinearColor Structure" :default (struct :`R` 1.0 :`G` 0.278321 :`A` 1.0)) (Scale :type "Float (double-precision)" :default 2.0))
  (bind _rendertexture (`self.RenderTexture`))
  (set `/Game/Robot_Dynamite/Effects/LCD/BP_LCD.Text` Text _rendertexture)
  (set `/Game/Robot_Dynamite/Effects/LCD/BP_LCD.Color` Color _rendertexture)
  (set `/Game/Robot_Dynamite/Effects/LCD/BP_LCD.Scale` Scale _rendertexture)
  (`MaterialInstanceDynamic.SetScalarParameterValue` (`self.Material`) "Scale" Scale)
  (`CanvasRenderTarget2D.UpdateResource` _rendertexture)
  (return))