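; BP_LCD is a canvas render target Blueprint that draws a text string for the Robot Dynamite LCD effect.
; Its Update event draws the Text variable with the given Font and Color, centered on the canvas with a one-pixel offset.
; GetStringDimensions estimates the text's size for centering by splitting the string and assuming fixed 16-pixel character cells, rather than measuring the font.
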(event `self.ReceiveUpdate`
  (params (Canvas :type "Canvas Object Reference") (Width :type Integer) (Height :type Integer))
  (bind _returnvalue (`KismetTextLibrary.Conv_TextToString` (`self.Text`)))
  (bind (_width _height) (`self.Get String Dimensions` _returnvalue))
  (`Canvas.K2_DrawText` Canvas (`self.Font`) _returnvalue (`KismetMathLibrary.MakeVector2D` (- (- (* Width 0.5) (* _width 0.5)) 1.0) (- (- (* Height 0.5) (* _height 0.5)) 1.0)) (`self.Color`) 0.0 (struct :`A` 1.0) (1.0 1.0) false false false (struct :`A` 1.0)))

(fn `Get String Dimensions`
  (params (SourceString :type String))
  (returns (Width :type "Float (double-precision)") (Height :type "Float (double-precision)"))
  (locals (W :type "Float (double-precision)") (H :type "Float (double-precision)"))
  (bind _returnvalue (`KismetStringLibrary.ParseIntoArray` SourceString " \n" false))
  (set `local.W` 0.0)
  (for _array_element _returnvalue
    (bind _output_get (set `local.W` (`KismetMathLibrary.FMax` (`local.W`) (`KismetMathLibrary.Conv_IntToDouble` (`KismetStringLibrary.Len` _array_element)))))
    (bind _output_get_2 (set `local.H` (`KismetMathLibrary.Conv_IntToDouble` (`KismetArrayLibrary.Array_Length` _returnvalue))))
    (return (* _output_get 16.0) (* _output_get_2 16.0))))