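; BP_LightSF_Controllable is a light fixture actor whose glowing mesh material follows the color and intensity of a controllable point light.
; On BeginPlay it passes brightness, hue and saturation channels plus the logarithmic-brightness setting to its BP_PointLight_Controllable child actor, initializes it and binds LightChanged.
; LightChanged drives a dynamic M_Light material's glow, keeping the light's hue and saturation and mapping clamped intensity logarithmically to value.
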(event `self.ReceiveBeginPlay`
  (bind _asbp_point_light_controllable (cast `/Game/Robot_Dynamite/Effects/Communication/BP_PointLight_Controllable` (`ChildActorComponent.ChildActor` (`self.Light`)) :!pure true))
  (set `/Game/Robot_Dynamite/Effects/Communication/BP_PointLight_Controllable.bLogarithmicBrightness` (`self.bLogarithmicBrightness`) _asbp_point_light_controllable)
  (set `/Game/Robot_Dynamite/Effects/Communication/BP_PointLight_Controllable.Brightness Channel` (`self.BrightnessChannel`) _asbp_point_light_controllable)
  (set `/Game/Robot_Dynamite/Effects/Communication/BP_PointLight_Controllable.Hue Channel` (`self.Hue Channel`) _asbp_point_light_controllable)
  (set `/Game/Robot_Dynamite/Effects/Communication/BP_PointLight_Controllable.Saturation Channel` (`self.Saturation Channel`) _asbp_point_light_controllable)
  (`/Game/Robot_Dynamite/Effects/Communication/BP_PointLight_Controllable.Init` _asbp_point_light_controllable)
  (add `/Game/Robot_Dynamite/Effects/Communication/BP_PointLight_Controllable.Light Changed` _asbp_point_light_controllable (delegate `Light Changed`)))

(event `Light Changed`
  (bind _light (`/Game/Robot_Dynamite/Effects/Communication/BP_PointLight_Controllable.Light` (cast `/Game/Robot_Dynamite/Effects/Communication/BP_PointLight_Controllable` (`ChildActorComponent.ChildActor` (`self.Light`)) :!pure true)))
  (bind (_h _s) (`KismetMathLibrary.RGBToHSV` (`LightComponentBase.GetLightColor` _light)))
  (bind _returnvalue (`PrimitiveComponent.CreateDynamicMaterialInstance` (`self.StaticMeshComponent`) 1 "/Game/Robot_Dynamite/Effects/Lighting/M_Light.M_Light"))
  (`MaterialInstanceDynamic.SetVectorParameterValue` _returnvalue "Light Glow" (`KismetMathLibrary.HSVToRGB` _h _s (/ (`KismetMathLibrary.Log` (`KismetMathLibrary.FClamp` (`LightComponentBase.Intensity` _light) 1.0 10000.0) 10.0) 4.0))))

(fn `UserConstructionScript`)