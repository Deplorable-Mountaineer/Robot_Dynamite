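; Scene component that moves itself along an array of waypoint actors toward a fractional target index, TargetFrame.
; Advance, Next, previous, Min and max set the target, and BeginPlay teleports to it.
; Tick steps Frame toward it at FrameRate and interpolates between neighboring waypoint transforms.
; A Circular flag switches from clamped linear travel to wraparound travel, with direction chosen by CircularDirection.
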(event `self.ReceiveBeginPlay`
  (bind _output_get (set `self.Frame` (`self.Normalize` (`self.Target Frame`))))
  (bind _output_get_2 (set `self.Target Frame` _output_get))
  (`self.K2_SetWorldTransform` (`self.Transform` _output_get_2) false true))

(event `self.ReceiveTick`
  (params (DeltaSeconds :type "Float (single-precision)"))
  (bind _frame (`self.Frame`))
  (if (not (`KismetMathLibrary.NearlyEqual_FloatFloat` (`self.Frame`) (`self.Target Frame`)))
    (set `self.Target Frame` (`self.Normalize` (`self.Target Frame`)))
    (`self.Update` DeltaSeconds)
    (`self.K2_SetWorldTransform` (`self.Transform` _frame))
    (`/Game/Robot_Dynamite/Base/BPML_Utilities_Components.Debug` (`KismetStringLibrary.Conv_DoubleToString` _frame) :!enabledstate Disabled)))

(event `Advance`
  (params (Amount :type "Float (double-precision)" :default 1.0))
  (set `self.Target Frame` (+ (`self.Target Frame`) Amount)))

(event `Next`
  (`self.Advance` 1.0))

(event `previous`
  (`self.Advance` -1.0))

(event `max`
  (set `self.Target Frame` (`KismetMathLibrary.Conv_IntToDouble` (- (`KismetArrayLibrary.Array_Length` (`self.Waypoints`)) 1))))

(event `Min`
  (set `self.Target Frame` 0.0))

(fn `CircularNearlyEqual`
  (params (A :type "Float (double-precision)") (A2 :type "Float (double-precision)") (ErrorTolerance :type "Float (double-precision)"))
  (returns (ReturnValue :type Boolean))
  (bind _returnvalue (`KismetArrayLibrary.Array_Length` (`self.Waypoints`)))
  (return (`KismetMathLibrary.NearlyEqual_FloatFloat` (`/Game/Robot_Dynamite/Base/BPFL_Utilities.CircularDistance` (`/Game/Robot_Dynamite/Base/BPFL_Utilities.CircularNormalize` A _returnvalue) (`/Game/Robot_Dynamite/Base/BPFL_Utilities.CircularNormalize` A2 _returnvalue) _returnvalue) 0.0 ErrorTolerance)))

(fn `GetCurrentFrame`
  (returns (Frame :type "Float (double-precision)"))
  (return (`self.Normalize` (`self.Frame`))))

(fn `Normalize`
  (params (InFrame :type "Float (double-precision)"))
  (returns (OutFrame :type "Float (double-precision)"))
  (return (select `bool` (`self.bCircular`) :`false` (`self.NormalizeLinear` InFrame) :`true` (`/Game/Robot_Dynamite/Base/BPFL_Utilities.CircularNormalize` InFrame (`KismetArrayLibrary.Array_Length` (`self.Waypoints`))))))

(fn `NormalizeLinear`
  (params (InFrame :type "Float (double-precision)"))
  (returns (OutFrame :type "Float (double-precision)"))
  (return (`KismetMathLibrary.FClamp` InFrame 0.0 (`KismetMathLibrary.Conv_IntToDouble` (- (`KismetArrayLibrary.Array_Length` (`self.Waypoints`)) 1)))))

(fn `Transform`
  (params (Frame :type "Float (double-precision)" :default 0.0))
  (returns (Transform :type "Transform Structure"))
  (bind _returnvalue (`KismetMathLibrary.FFloor` Frame))
  (bind _waypoints (`self.Waypoints`))
  (bind _waypoints_2 (`self.Waypoints`))
  (bind _returnvalue_2 (`KismetArrayLibrary.Array_Length` (`self.Waypoints`)))
  (bind _returnvalue_3 (`KismetMathLibrary.Conv_IntToDouble` _returnvalue))
  (if (`self.bCircular`)
    (return (`KismetMathLibrary.TLerp` (`Actor.GetTransform` (`|GetArrayItem` _waypoints (`KismetMathLibrary.Round` (`/Game/Robot_Dynamite/Base/BPFL_Utilities.CircularFloor` Frame _returnvalue_2)))) (`Actor.GetTransform` (`|GetArrayItem` _waypoints (`KismetMathLibrary.Round` (`/Game/Robot_Dynamite/Base/BPFL_Utilities.CircularCeil` Frame _returnvalue_2)))) (- Frame _returnvalue_3)))
    (else
      (return (`KismetMathLibrary.TLerp` (`Actor.GetTransform` (`|GetArrayItem` _waypoints_2 _returnvalue)) (`Actor.GetTransform` (`|GetArrayItem` _waypoints_2 (`KismetMathLibrary.FCeil` Frame))) (- Frame _returnvalue_3))))))

(fn `Update`
  (params (DeltaTime :type "Float (double-precision)"))
  (if (`self.bCircular`)
    (`self.UpdateCircular` DeltaTime)
    (else
      (`self.UpdateLinear` DeltaTime)))
  (return))

(fn `UpdateCircular`
  (params (DeltaTime :type "Float (double-precision)"))
  (bind _returnvalue (* (`self.FrameRate`) DeltaTime))
  (if (`self.CircularNearlyEqual` (`self.Frame`) (`self.Target Frame`) _returnvalue)
    (set `self.Frame` (`/Game/Robot_Dynamite/Base/BPFL_Utilities.CircularNormalize` (`self.Target Frame`) (`KismetArrayLibrary.Array_Length` (`self.Waypoints`))))
    (else
      (if (`/Game/Robot_Dynamite/Base/BPFL_Utilities.CircularDirection` (`self.Frame`) (`self.Target Frame`) (`KismetArrayLibrary.Array_Length` (`self.Waypoints`)))
        (set `self.Frame` (`/Game/Robot_Dynamite/Base/BPFL_Utilities.CircularNormalize` (+ (`self.Frame`) (* (`self.FrameRate`) DeltaTime)) (`KismetArrayLibrary.Array_Length` (`self.Waypoints`))))
        (else
          (set `self.Frame` (`/Game/Robot_Dynamite/Base/BPFL_Utilities.CircularNormalize` (- (`self.Frame`) _returnvalue) (`KismetArrayLibrary.Array_Length` (`self.Waypoints`))))))
      (return))))

(fn `UpdateLinear`
  (params (DeltaTime :type "Float (double-precision)"))
  (bind _returnvalue (* DeltaTime (`self.FrameRate`)))
  (if (`KismetMathLibrary.NearlyEqual_FloatFloat` (`self.Frame`) (`self.Target Frame`) _returnvalue)
    (set `self.Frame` (`self.Target Frame`))
    (return)
    (else
      (set `self.Frame` (+ (* (`KismetMathLibrary.SignOfFloat` (- (`self.Target Frame`) (`self.Frame`))) _returnvalue) (`self.Frame`)))
      (return))))