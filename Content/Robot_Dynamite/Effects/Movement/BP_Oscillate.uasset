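; BP_Oscillate is a movement effect that swings its relative rotation back and forth between StartAngle and StopAngle around a configurable Axis.
; Each Tick maps a sine of game time to a lerp alpha and builds the rotation from the axis and resulting angle.
; Dividing the phase by the angle range makes Rate the average angular speed in degrees per second, with smooth easing at both ends.
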(event `self.ReceiveTick`
  (params (DeltaSeconds :type "Float (single-precision)"))
  (`self.K2_SetRelativeRotation` (`KismetMathLibrary.RotatorFromAxisAndAngle` (`self.Axis`) (`KismetMathLibrary.Lerp` (`self.StartAngle`) (`self.StopAngle`) (/ (+ (`KismetMathLibrary.DegSin` (/ (* (`KismetSystemLibrary.GetGameTimeInSeconds`) (`self.Rate`) 180.0) (- (`self.StopAngle`) (`self.StartAngle`)))) 1.0) 2.0)))))