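; A multi-position switch that a player-controlled operator steps to the next position.
; Every change goes through SetCurrentPosition, which wraps or clamps the value, broadcasts it as an integer on the transceiver channel and refreshes the visuals.
; A text display shows the position in a color blended between off and on, while the toggle mesh tilts at either extreme.
; It can also be set remotely by integers received on its AutoSetFromChannel.
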(event `Fully Off`
  ;[0.2471 0.2118 0.1804] State
  (`self.SetCurrentPosition` 0))

(event `Next`
  ;[0.2471 0.2118 0.1804] State
  (`self.Advance` 1))

(event `Fully On`
  ;[0.2471 0.2118 0.1804] State
  (`self.SetCurrentPosition` (- (`self.NumPositions`) 1)))

(event `self.ReceiveBeginPlay`
  ;[0 1 0.5] Startup
  (bind _output_get (set `self.CurrentPosition` (`self.StartPosition`)))
  (`self.Set Visuals` _output_get)
  (`/Game/Robot_Dynamite/Effects/Communication/BP_TransceiverComponent.Tune In Integer` (`self.BP_Transceiver`) (`self.Auto Set From Channel`)))

(event `Previous`
  ;[0.2471 0.2118 0.1804] State
  (`self.Advance` -1))

(event `Advance`
  (params (Amount :type Integer :default 1))
  ;[0.2471 0.2118 0.1804] State
  (`self.SetCurrentPosition` (+ (`self.CurrentPosition`) Amount)))

(event `Set Visuals`
  (params (Position :type Integer))
  ;[0.04971 0.03689 0.02732] Set Toggle And Display
  (`TextRenderComponent.K2_SetText` (`self.Display`) (`KismetTextLibrary.Conv_IntToText` Position))
  (`TextRenderComponent.SetTextRenderColor` (`self.Display`) (`KismetMathLibrary.Conv_LinearColorToColor` (`KismetMathLibrary.LinearColorLerp` (`KismetMathLibrary.Conv_ColorToLinearColor` (`self.Full Off Color`)) (`KismetMathLibrary.Conv_ColorToLinearColor` (`self.Full On Color`)) (/ (`KismetMathLibrary.Conv_IntToDouble` Position) (`KismetMathLibrary.Conv_IntToDouble` (- (`self.NumPositions`) 1))))))
  (if (== Position (- (`self.NumPositions`) 1))
    (`SceneComponent.K2_SetRelativeRotation` (`self.Toggle Mesh`) (struct :`Roll` -30.0) false false)
    (elif (== Position 0)
      (`SceneComponent.K2_SetRelativeRotation` (`self.Toggle Mesh`) (struct :`Roll` 30.0) false false)
      (else
        (`SceneComponent.K2_SetRelativeRotation` :`self` (`self.Toggle Mesh`))))))

(event `self.BP_Transceiver.Integer Received`
  (bind _value (`/Game/Robot_Dynamite/Effects/Communication/BP_TransceiverComponent.Receive Integer` (`self.BP_Transceiver`) "None"))
  (`self.SetCurrentPosition` _value))

(fn `GetCurrentPosition`
  (returns (Position :type Integer))
  (return (`self.CurrentPosition`)))

(fn `Operate`
  (params (Operator :type "/Game/Robot_Dynamite/Characters/BP_Character Object Reference"))
  (returns (Success :type Boolean))
  (if (`Pawn.IsPlayerControlled` Operator)
    (`self.Next`)
    (return true)
    (else
      (return false))))

(fn `SetCurrentPosition`
  (params (`New Position` :type Integer :default 0))
  (returns (`Actual New Position` :type Integer))
  (bind _numpositions (`self.NumPositions`))
  (bind _output_get (set `self.CurrentPosition` (select `bool` (`self.bCircular`) :`false` (`KismetMathLibrary.Clamp` `New Position` 0 (- (`self.NumPositions`) 1)) :`true` (mod (+ (mod `New Position` _numpositions) _numpositions) _numpositions))))
  (`/Game/Robot_Dynamite/Effects/Communication/BP_TransceiverComponent.Send Integer` (`self.BP_Transceiver`) (`self.Channel`) _output_get)
  (`self.Set Visuals` _output_get)
  (return _output_get))

(fn `UserConstructionScript`
  (bind _output_get (set `self.CurrentPosition` (`self.StartPosition`)))
  (`self.Set Visuals` _output_get))