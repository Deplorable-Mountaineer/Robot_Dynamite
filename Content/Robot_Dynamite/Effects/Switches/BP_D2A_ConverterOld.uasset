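; BP_D2A_ConverterOld is a switch effect that converts a discrete switch position into a numeric value.
; Notify reads the position from a BP_SwitchOld sender and stores it, either wrapped or clamped to the setting count.
; GetResult maps the stored setting by linear, exponential, lookup table with default, or overridable-style pass-through custom function.
; The A*x+B mode actually calls the exponential formula, leaving AxB unused.
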(event `/Game/Robot_Dynamite/Base/BPI_Notify_Receiver.Notify`
  (params (Sender :type "Actor Object Reference"))
  (`self.Set Current Setting` (`/Game/Robot_Dynamite/Effects/Switches/BP_SwitchOld.GetCurrentPosition` (cast `/Game/Robot_Dynamite/Effects/Switches/BP_SwitchOld` Sender :!pure true))))

(fn `A*B^x+C`
  (params (Value :type "Float (double-precision)"))
  (returns (`Return Value` :type "Float (double-precision)"))
  (return (+ (* (`self.A`) (`KismetMathLibrary.MultiplyMultiply_FloatFloat` (`self.B`) Value)) (`self.C`))))

(fn `Ax+B`
  (params (Value :type "Float (double-precision)"))
  (returns (`Return Value` :type "Float (double-precision)"))
  (return (+ (* Value (`self.A`)) (`self.B`))))

(fn `CustomFunction`
  (params (In :type "Float (double-precision)"))
  (returns (Out :type "Float (double-precision)"))
  (return In))

(fn `GetResult`
  (returns (Result :type "Float (double-precision)"))
  (bind _current_setting (`self.Current Setting`))
  (bind _returnvalue (`KismetMathLibrary.Conv_IntToDouble` _current_setting))
  (switch `/Game/Robot_Dynamite/Effects/Switches/EConvertMethod` (`self.Convert Method`)
    (:`NewEnumerator0`
      (bind _returnvalue_2 (`self.Linear_0_to_A` _returnvalue))
      (return _returnvalue_2))
    (:`NewEnumerator1`
      (bind _return_value (`self.A*B^x+C` _returnvalue))
      (return _return_value))
    (:`NewEnumerator2`
      (bind _return_value_2 (`self.A*B^x+C` _returnvalue))
      (return _return_value_2))
    (:`NewEnumerator3`
      (bind _return_value_3 (`self.Use LUT` _current_setting))
      (return _return_value_3))
    (:`NewEnumerator4`
      (bind _out (`self.CustomFunction` _returnvalue))
      (return _out))))

(fn `Linear_0_to_A`
  (params (Value :type "Float (double-precision)"))
  (returns (ReturnValue :type "Float (double-precision)"))
  (return (* (/ Value (`KismetMathLibrary.Conv_IntToDouble` (- (`self.Num Settings`) 1))) (`self.A`))))

(fn `Set Current Setting`
  (params (Value :type Integer :default 1))
  (returns (`Current Setting` :type Integer))
  (bind _num_settings (`self.Num Settings`))
  (bind _output_get (set `self.Current Setting` (select `bool` (`self.bCircular`) :`false` (`KismetMathLibrary.Clamp` Value 0 (- (`self.Num Settings`) 1)) :`true` (mod (+ (mod Value _num_settings) _num_settings) _num_settings))))
  (return _output_get))

(fn `Use LUT`
  (params (Value :type Integer))
  (returns (`Return Value` :type "Float (double-precision)"))
  (bind (_value _returnvalue) (`BlueprintMapLibrary.Map_Find` (`self.LUT`) Value))
  (return (select `bool` _returnvalue :`false` (`self.A`) :`true` _value)))

(fn `UserConstructionScript`)