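; BP_SwitchConverterOld is a switch that converts another switch's position into an all-or-nothing position of its own.
; It subscribes to the Input switch on BeginPlay, though its Notify handler is empty.
; GetCurrentPosition reads Input on demand and returns the last position when the value lies between AtLeast and AtMost and passes optional Odd or Even filters, otherwise zero.
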(event `self.ReceiveBeginPlay`
  (`parent.ReceiveBeginPlay`)
  (`/Game/Robot_Dynamite/Base/BPI_Notify_Sender.Subscribe` (`self.Input`) self))

(event `/Game/Robot_Dynamite/Base/BPI_Notify_Receiver.Notify`
  (params (Sender :type "Actor Object Reference")))

(fn `GetCurrentPosition`
  (returns (Position :type Integer))
  (bind _position (`self.GetCurrentPosition` (`self.Input`)))
  (bind _returnvalue (mod _position 2))
  (return (select `bool` (and (>= _position (`self.At Least`)) (<= _position (`self.At Most`)) (or (not (`self.bOdd`)) (== _returnvalue 1)) (or (not (`self.bEven`)) (== _returnvalue 0))) :`true` (- (`self.NumPositions`) 1))))

(fn `UserConstructionScript`
  (`parent.UserConstructionScript`))