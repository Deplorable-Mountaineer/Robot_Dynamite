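; BP_CardSlot is a switch operated with a key item of the required class from the operator's inventory.
; Operate consumes that item when switching on, refuses if it is missing, and respawns it in the inventory when operating an active slot without holding one.
; State changes rebuild the slot's children, attaching the key as a child actor at the "Key" socket when on, and swap the LED material.
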(event `self.On State Change`
  (params (Position :type "Float (single-precision)"))
  (`parent.On State Change` Position)
  (for _array_element (`SceneComponent.GetChildrenComponents` (`self.CardSlot`) true)
    (`ActorComponent.K2_DestroyComponent` _array_element))
  (if (> Position 0.0)
    (bind _returnvalue (`AddComponent|NODE_AddChildActorComponent-0` :`bManualAttachment` true :`RelativeTransform` (`KismetMathLibrary.MakeTransform` (0.0 0.0 0.0))))
    (`ChildActorComponent.SetChildActorClass` _returnvalue (`self.Key Required`))
    (`SceneComponent.K2_AttachToComponent` _returnvalue (`self.CardSlot`) "Key" "KeepRelative" "KeepRelative" "KeepRelative" true)
    (`PrimitiveComponent.SetMaterial` (`self.CardSlot`) 4 "/Game/Robot_Dynamite/Environment/Props/LightsEffects/MI_LedTextMat.MI_LedTextMat")
    (else
      (`PrimitiveComponent.SetMaterial` (`self.CardSlot`) 4 "/Game/Robot_Dynamite/Environment/Props/LightsEffects/MI_LedDStick.MI_LedDStick"))))

(fn `Operate`
  (params (Operator :type "/Game/Robot_Dynamite/Characters/BP_Character Object Reference"))
  (returns (Success :type Boolean))
  (bind _bp_inventory (`/Game/Robot_Dynamite/Characters/BP_Character.BP_Inventory` Operator))
  (bind (_item _isvalid _slot) (`/Game/Robot_Dynamite/Inventory/BP_Inventory.GetItem` _bp_inventory (`self.Key Required`)))
  (if _isvalid
    (if (> (`self.Get Position`) 0.0)
      (bind _success (`parent.Operate` Operator))
      (return _success)
      (else
        (`self.K2_DestroyActor` _item)
        (set `/Game/Robot_Dynamite/Inventory/BP_Slot.Item` null _slot)
        (bind _success_2 (`parent.Operate` Operator))
        (return _success_2)))
    (elif (> (`self.Get Position`) 0.0)
      (bind _success_3 (`parent.Operate` Operator))
      (`/Game/Robot_Dynamite/Inventory/BP_Inventory.SpawnInventoryItem` _bp_inventory (`self.Key Required`) _slot Operator (`/Game/Robot_Dynamite/Inventory/BP_Slot.Socket` _slot))
      (return _success_3)
      (else
        (return false)))))

(fn `UserConstructionScript`
  (`parent.UserConstructionScript`))