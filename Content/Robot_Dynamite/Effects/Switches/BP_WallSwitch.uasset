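; BP_WallSwitch is a wall switch with a pivoting toggle and an LCD display that shows its current position as a number.
; BeginPlay binds the LCD component to a material slot on the switch plate mesh, initializes it and shows the starting position in orange.
; On each state change, the toggle's pitch is interpolated across the Min to Max range and, once the display is ready, the LCD text is refreshed.
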(event `self.ReceiveBeginPlay`
  (bind _bp_lcd_component (`self.BP_LCD_Component`))
  (`parent.ReceiveBeginPlay`)
  (set `/Game/Robot_Dynamite/Effects/LCD/BP_LCD_Component.LCD Mesh Component` (`self.SwitchPlate`) _bp_lcd_component)
  (set `/Game/Robot_Dynamite/Effects/LCD/BP_LCD_Component.LCD Material Index` 2 _bp_lcd_component)
  (`/Game/Robot_Dynamite/Effects/LCD/BP_LCD_Component.Init` _bp_lcd_component)
  (`/Game/Robot_Dynamite/Effects/LCD/BP_LCD_Component.SetRenderTextureParameters` _bp_lcd_component (`KismetTextLibrary.Conv_DoubleToText` (`self.Get Position`) "HalfFromZero" true 1 4 0 2) (struct :`R` 1.0 :`G` 0.278321 :`A` 1.0) 4.0)
  (set `self.bReady` true))

(event `self.On State Change`
  (params (Position :type "Float (single-precision)"))
  (`SceneComponent.K2_SetRelativeRotation` (`self.Toggle`) (`KismetMathLibrary.RLerp` (struct :`Roll` 30.0) (struct :`Roll` -30.0) (/ (- Position (`self.Min`)) (- (`self.Max`) (`self.Min`)))) false false)
  (if (`self.bReady`)
    (`/Game/Robot_Dynamite/Effects/LCD/BP_LCD_Component.SetRenderTextureParameters` (`self.BP_LCD_Component`) (`KismetTextLibrary.Conv_DoubleToText` Position "HalfFromZero" true 1 4 0 2) (struct :`R` 1.0 :`G` 0.278321 :`A` 1.0) 4.0)))

(fn `UserConstructionScript`
  (`parent.UserConstructionScript`))