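; BP_Switch is a multi-position switch actor that shows its position through a toggle mesh and a colored number display.
; Next, Previous, FullyOn, FullyOff and Advance all route through SetCurrentPosition, which either wraps or clamps the value depending on the Circular flag.
; Each set notifies subscribed receivers via NotifyMessage, then tilts the toggle and tints the text between off and on colors in HSV.
; The construction script and BeginPlay apply StartPosition without notifying subscribers.
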(event `Fully Off`
  ;[0.2471 0.2118 0.1804] State
  (`self.SetCurrentPosition` 0))

(event `Next`
  ;[0.2471 0.2118 0.1804] State
  (`self.Advance` 1))

(event `Fully On`
  ;[0.2471 0.2118 0.1804] State
  (`self.SetCurrentPosition` (- (`self.NumPositions`) 1)))

(event `Previous`
  ;[0.2471 0.2118 0.1804] State
  (`self.Advance` -1))

(event `Advance`
  (params (Amount :type Integer :default 1))
  ;[0.2471 0.2118 0.1804] State
  (`self.SetCurrentPosition` (+ (`self.CurrentPosition`) Amount)))

(event `self.ReceiveBeginPlay`
  ;[0 1 0.5] Startup
  (bind _output_get (set `self.CurrentPosition` (`self.StartPosition`)))
  (`self.On New Position` _output_get))

(event `NotifyAll`
  ;[0.04971 0.03689 0.02732] Messages
  (for _array_element (`self.Subscribers`)
    (message `/Game/Robot_Dynamite/Base/BPI_Notify_Receiver.Notify` _array_element self)))

(event `/Game/Robot_Dynamite/Base/BPI_Notify_Sender.Subscribe`
  (params (Receiver :type "Actor Object Reference"))
  ;[0.04971 0.03689 0.02732] Messages
  (`KismetArrayLibrary.Array_AddUnique` (`self.Subscribers`) Receiver))

(event `/Game/Robot_Dynamite/Base/BPI_Notify_Sender.Unsubscribe`
  (params (Receiver :type "Actor Object Reference"))
  ;[0.04971 0.03689 0.02732] Messages
  (`KismetArrayLibrary.Array_RemoveItem` (`self.Subscribers`) Receiver))

(event `On New Position`
  (params (Position :type Integer))
  ;[0.04971 0.03689 0.02732] Set Toggle And Display
  (`TextRenderComponent.K2_SetText` (`self.Display`) (`KismetTextLibrary.Conv_IntToText` Position))
  (`TextRenderComponent.SetTextRenderColor` (`self.Display`) (`KismetMathLibrary.Conv_LinearColorToColor` (`KismetMathLibrary.LinearColorLerpUsingHSV` (`KismetMathLibrary.Conv_ColorToLinearColor` (`self.Full Off Color`)) (`KismetMathLibrary.Conv_ColorToLinearColor` (`self.Full On Color`)) (/ (`KismetMathLibrary.Conv_IntToDouble` Position) (`KismetMathLibrary.Conv_IntToDouble` (- (`self.NumPositions`) 1))))))
  (if (== Position (- (`self.NumPositions`) 1))
    (`SceneComponent.K2_SetRelativeRotation` (`self.Toggle Mesh`) (struct :`Roll` -30.0) false false)
    (elif (== Position 0)
      (`SceneComponent.K2_SetRelativeRotation` (`self.Toggle Mesh`) (struct :`Roll` 30.0) false false)
      (else
        (`SceneComponent.K2_SetRelativeRotation` (`self.Toggle Mesh`) (struct) false false)))))

(fn `GetCurrentPosition`
  (returns (NewParam :type Integer))
  (return (`self.CurrentPosition`)))

(fn `SetCurrentPosition`
  (params (`New Position` :type Integer :default 0))
  (returns (`Actual New Position` :type Integer))
  (bind _numpositions (`self.NumPositions`))
  (bind _output_get (set `self.CurrentPosition` (select `bool` (`self.bCircular`) :`false` (`KismetMathLibrary.Clamp` `New Position` 0 (- (`self.NumPositions`) 1)) :`true` (mod (+ (mod `New Position` _numpositions) _numpositions) _numpositions))))
  (`self.NotifyAll`)
  (`self.On New Position` _output_get)
  (return _output_get))

(fn `UserConstructionScript`
  (bind _output_get (set `self.CurrentPosition` (`self.StartPosition`)))
  (`self.On New Position` _output_get))