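; Switch adapter that combines several input switches into one switch position, acting as a configurable logic gate.
; It subscribes to its input switches on BeginPlay and caches their positions in four maps by role: Sum, Sum Negative, Product, Product Not.
; Each notification refreshes the maps and recomputes the output.
; A positive net sum wins; otherwise any product inputs are multiplied, with nonzero Product Not inputs forcing zero.
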(event `self.ReceiveBeginPlay`
  (`parent.ReceiveBeginPlay`)
  (`self.SolicitSubscriptionsFromSwitches`)
  (bind _newstate (`self.ComputeState`))
  (`self.SetCurrentPosition` _newstate))

(event `/Game/Robot_Dynamite/Base/BPI_Notify_Receiver.Notify`
  (params (Sender :type "Actor Object Reference"))
  (`self.UpdateSwitchStates`)
  (bind _newstate (`self.ComputeState`))
  (`self.SetCurrentPosition` _newstate))

(fn `ComputeState`
  (returns (NewState :type Integer))
  (locals (State :type Integer))
  (bind _values (`BlueprintMapLibrary.Map_Values` (`self.Sum`)))
  (for _array_element _values
    (bind _output_get (set `local.State` (+ _array_element (`local.State`))))
    (`/Game/Robot_Dynamite/Base/BPML_Utilities_Actors.Debug` false "sum:" (`KismetStringLibrary.Conv_IntToString` _output_get)))
  (bind _values_2 (`BlueprintMapLibrary.Map_Values` (`self.SumNegative`)))
  (for _array_element_2 _values_2
    (bind _output_get_2 (set `local.State` (- (`local.State`) _array_element_2)))
    (`/Game/Robot_Dynamite/Base/BPML_Utilities_Actors.Debug` false "inv sum:" (`KismetStringLibrary.Conv_IntToString` _output_get_2)))
  (if (or (> (`local.State`) 0) (== (+ (`BlueprintMapLibrary.Map_Length` (`self.Product`)) (`BlueprintMapLibrary.Map_Length` (`self.ProductNot`))) 0))
    (return (`local.State`))
    (else
      (set `local.State` 1)
      (bind _values_3 (`BlueprintMapLibrary.Map_Values` (`self.Product`)))
      (for _array_element_3 _values_3
        (bind _output_get_3 (set `local.State` (* _array_element_3 (`local.State`))))
        (if (== _output_get_3 0)
          (break)
          (else
            (`/Game/Robot_Dynamite/Base/BPML_Utilities_Actors.Debug` false "Product:" (`KismetStringLibrary.Conv_IntToString` _output_get_3)))))
      (bind _values_4 (`BlueprintMapLibrary.Map_Values` (`self.ProductNot`)))
      (for _array_element_4 _values_4
        (bind _output_get_4 (set `local.State` (select `bool` (== _array_element_4 0) :`true` (`local.State`))))
        (if (== _output_get_4 0)
          (break)
          (else
            (`/Game/Robot_Dynamite/Base/BPML_Utilities_Actors.Debug` false "Neg Product:" (`KismetStringLibrary.Conv_IntToString` _output_get_4)))))
      (return (`local.State`)))))

(fn `SolicitSubscriptionsFromSwitches`
  (for _array_element (`self.InputSwitches`)
    (`self.Subscribe` (break `/Game/Robot_Dynamite/Effects/Switches/SSenderConfigMulti` _array_element) self)
    (switch `/Game/Robot_Dynamite/Effects/Switches/ESwitchCombinationMethod` (`.Config_6_436AAD704CD183D9E73BF495922F832B` (break `/Game/Robot_Dynamite/Effects/Switches/SSenderConfigMulti` _array_element))
      (:`NewEnumerator0`
        (bind _position (`self.GetCurrentPosition` (break `/Game/Robot_Dynamite/Effects/Switches/SSenderConfigMulti` _array_element)))
        (`BlueprintMapLibrary.Map_Add` (`self.Product`) (break `/Game/Robot_Dynamite/Effects/Switches/SSenderConfigMulti` _array_element) _position))
      (:`NewEnumerator1`
        (`BlueprintMapLibrary.Map_Add` (`self.Sum`) (break `/Game/Robot_Dynamite/Effects/Switches/SSenderConfigMulti` _array_element) _position))
      (:`NewEnumerator7`
        (`BlueprintMapLibrary.Map_Add` (`self.ProductNot`) (break `/Game/Robot_Dynamite/Effects/Switches/SSenderConfigMulti` _array_element) _position))
      (:`NewEnumerator8`
        (`BlueprintMapLibrary.Map_Add` (`self.SumNegative`) (break `/Game/Robot_Dynamite/Effects/Switches/SSenderConfigMulti` _array_element) _position))))
  (return))

(fn `UpdateSwitchStates`
  (for _array_element (`self.InputSwitches`)
    (switch `/Game/Robot_Dynamite/Effects/Switches/ESwitchCombinationMethod` (`.Config_6_436AAD704CD183D9E73BF495922F832B` (break `/Game/Robot_Dynamite/Effects/Switches/SSenderConfigMulti` _array_element))
      (:`NewEnumerator0`
        (bind _position (`self.GetCurrentPosition` (break `/Game/Robot_Dynamite/Effects/Switches/SSenderConfigMulti` _array_element)))
        (`BlueprintMapLibrary.Map_Add` (`self.Product`) (break `/Game/Robot_Dynamite/Effects/Switches/SSenderConfigMulti` _array_element) _position))
      (:`NewEnumerator1`
        (`BlueprintMapLibrary.Map_Add` (`self.Sum`) (break `/Game/Robot_Dynamite/Effects/Switches/SSenderConfigMulti` _array_element) _position))
      (:`NewEnumerator7`
        (`BlueprintMapLibrary.Map_Add` (`self.ProductNot`) (break `/Game/Robot_Dynamite/Effects/Switches/SSenderConfigMulti` _array_element) _position))
      (:`NewEnumerator8`
        (`BlueprintMapLibrary.Map_Add` (`self.SumNegative`) (break `/Game/Robot_Dynamite/Effects/Switches/SSenderConfigMulti` _array_element) _position))))
  (return))

(fn `UserConstructionScript`)