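; BP_CountingTrigger is a trigger actor that counts when the robot player, BP_RobotDynamite, enters it.
; On overlap while Enabled, it displays its TextOnTrigger message on the robot in orange.
; It then increments the tally for its Type in the BP_GameState SpecialAreas map, starting from zero if the key is absent.
; With Once set, it disables itself after the first counted overlap.
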(event `self.ReceiveActorBeginOverlap`
  (params (OtherActor :type "Actor Object Reference"))
  (bind _special_areas (`/Game/Robot_Dynamite/Base/GameFramework/BP_GameState.Special Areas` (cast `/Game/Robot_Dynamite/Base/GameFramework/BP_GameState` (`GameplayStatics.GetGameState`) :!pure true)))
  (bind (_value _returnvalue) (`BlueprintMapLibrary.Map_Find` _special_areas (`self.Type`)))
  (if (`self.bEnabled`)
    (bind _asbp_robot_dynamite (cast `/Game/Robot_Dynamite/Characters/Player/BP_RobotDynamite` OtherActor))
    (`/Game/Robot_Dynamite/Characters/Player/BP_RobotDynamite.DisplayMessage` _asbp_robot_dynamite (`KismetTextLibrary.Conv_TextToString` (`self.TextOnTrigger`)) (struct :`R` 1.0 :`G` 0.278321 :`A` 1.0))
    (`BlueprintMapLibrary.Map_Add` _special_areas (`self.Type`) (+ (select `bool` _returnvalue :`true` _value) 1))
    (if (`self.bOnce`)
      (set `self.bEnabled` false))))

(fn `UserConstructionScript`)