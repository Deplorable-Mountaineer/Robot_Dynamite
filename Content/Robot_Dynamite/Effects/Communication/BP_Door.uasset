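; A lockable double door that characters open by overlapping its trigger or operating it, with optional delayed auto-close.
; BP_Transceiver float channels remotely set the lock state and, while unlocked, the target open amount.
; Tick steps openness toward that target over OpenTime, lerping both panels between closed and open sockets on the frame.
; Panels hitting a character while sufficiently open reopen fully, then restore the channel's value after a delay.
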(event `self.ReceiveBeginPlay`
  (`self.Reset`))

(event `self.ReceiveTick`
  (params (DeltaSeconds :type "Float (single-precision)"))
  (bind _returnvalue (/ DeltaSeconds (`self.Open Time`)))
  (`|ExecutionSequence`
    (:`then_0`
      (if (`self.bAutoClose`)
        (set `self.bAutoClose` false)
        (`KismetSystemLibrary.Delay` (`self.Trigger Close Delay`))
        (set `self.New Open Amount` 0.0)))
    (:`then_1`
      (if (not (`KismetMathLibrary.NearlyEqual_FloatFloat` (`self.Open Amount`) (`self.New Open Amount`)))
        (if (< (`self.Open Amount`) (`self.New Open Amount`))
          (set `self.Open Amount` (+ (`self.Open Amount`) _returnvalue))
          (if (not (< (`self.Open Amount`) (`self.New Open Amount`)))
            (set `self.Open Amount` (`self.New Open Amount`)))
          (else
            (set `self.Open Amount` (- (`self.Open Amount`) _returnvalue))
            (if (< (`self.Open Amount`) (`self.New Open Amount`))
              (set `self.Open Amount` (`self.New Open Amount`)))))
        (`self.AdjustDoorOpenness`)))))

(event `self.BP_Transceiver.Float Received`
  ;[1 0.2783 0] Remote Control
  (bind (_value _channel_exists) (`/Game/Robot_Dynamite/Effects/Communication/BP_TransceiverComponent.Receive Float` (`self.BP_Transceiver`) (`self.Unlock Channel`)))
  (if _channel_exists
    (set `self.bUnlocked` (> _value 0.0001)))
  (bind (_value_2 _channel_exists_2) (`/Game/Robot_Dynamite/Effects/Communication/BP_TransceiverComponent.Receive Float` (`self.BP_Transceiver`) (`self.Input Channel`)))
  (if (and _channel_exists_2 (`self.bUnlocked`))
    (set `self.New Open Amount` _value_2)))

(event `self.LeftDoor.OnComponentHit`
  (params (HitComponent :type "PrimitiveComponent Object Reference") (OtherActor :type "Actor Object Reference") (OtherComp :type "PrimitiveComponent Object Reference") (NormalImpulse :type "Vector Structure") (Hit :type "HitResult Structure (by ref)"))
  ;[1 0.2783 0] Safety Auto Reopen When Blocked By Character
  (cast `/Game/Robot_Dynamite/Characters/BP_Character` OtherActor)
  (if (>= (`self.Open Amount`) 0.1) :!label _label
    (set `self.New Open Amount` 1.0)
    (`KismetSystemLibrary.Delay` (`self.Open Time`))
    (bind (_value _channel_exists) (`/Game/Robot_Dynamite/Effects/Communication/BP_TransceiverComponent.Receive Float` (`self.BP_Transceiver`) (`self.Input Channel`)))
    (if _channel_exists
      (set `self.New Open Amount` _value))))

(event `self.RightDoor.OnComponentHit`
  (params (HitComponent :type "PrimitiveComponent Object Reference") (OtherActor :type "Actor Object Reference") (OtherComp :type "PrimitiveComponent Object Reference") (NormalImpulse :type "Vector Structure") (Hit :type "HitResult Structure (by ref)"))
  ;[1 0.2783 0] Safety Auto Reopen When Blocked By Character
  (cast `/Game/Robot_Dynamite/Characters/BP_Character` OtherActor)
  (goto _label))

(event `self.Trigger.OnComponentBeginOverlap`
  (params (OverlappedComponent :type "PrimitiveComponent Object Reference") (OtherActor :type "Actor Object Reference") (OtherComp :type "PrimitiveComponent Object Reference") (OtherBodyIndex :type Integer) (bFromSweep :type Boolean) (SweepResult :type "HitResult Structure (by ref)"))
  (bind _success (`self.OpenDoor` OtherActor))
  (if (and _success (> (`self.Trigger Close Delay`) 0.0))
    (set `self.bAutoClose` true)))

(fn `AdjustDoorOpenness`
  (bind _frame (`self.Frame`))
  (bind _open_amount (`self.Open Amount`))
  (`SceneComponent.K2_SetWorldTransform` (`self.LeftDoor`) (`KismetMathLibrary.TLerp` (`SceneComponent.GetSocketTransform` _frame "Left Door Closed" "RTS_World") (`SceneComponent.GetSocketTransform` _frame "Left Door Open" "RTS_World") _open_amount) false false)
  (`SceneComponent.K2_SetWorldTransform` (`self.RightDoor`) (`KismetMathLibrary.TLerp` (`SceneComponent.GetSocketTransform` _frame "Right Door Closed" "RTS_World") (`SceneComponent.GetSocketTransform` _frame "Right Door Open" "RTS_World") _open_amount) false false))

(fn `OpenDoor`
  (params (Operator :type "Object Object Reference"))
  (returns (Success :type Boolean))
  (bind _asbp_character (cast `/Game/Robot_Dynamite/Characters/BP_Character` Operator)
    (:`then`
      (bind _returnvalue (`Pawn.IsPlayerControlled` _asbp_character))
      (if (and _returnvalue (not (`self.bUnlocked`)))
        (`/Game/Robot_Dynamite/Base/BPML_Utilities_Actors.DisplayMessage` "Door is locked!" (struct :`R` 0.424385 :`G` 0.040803 :`B` 0.040803 :`A` 1.0))
        (return false)
        (elif (and (or (and _returnvalue (`self.bPlayerOverlaps`)) (`self.bCharacterOverlaps`)) (`self.bUnlocked`))
          (set `self.New Open Amount` 1.0)
          (return true)
          (else
            (return false)))))
    (:`CastFailed`
      (return false))))

(fn `Operate`
  (params (Operator :type "/Game/Robot_Dynamite/Characters/BP_Character Object Reference"))
  (returns (Success :type Boolean))
  (bind _success (`self.OperateDoor` Operator))
  (set `self.bAutoClose` true)
  (return _success))

(fn `OperateDoor`
  (params (Operator :type "Object Object Reference"))
  (returns (Success :type Boolean))
  (bind _asbp_character (cast `/Game/Robot_Dynamite/Characters/BP_Character` Operator)
    (:`then`
      (bind _returnvalue (`Pawn.IsPlayerControlled` _asbp_character))
      (if (and _returnvalue (not (`self.bUnlocked`)))
        (`/Game/Robot_Dynamite/Base/BPML_Utilities_Actors.DisplayMessage` "Door is locked!" (struct :`R` 0.424385 :`G` 0.040803 :`B` 0.040803 :`A` 1.0))
        (return true)
        (elif (and (or (and _returnvalue (`self.bPlayerOperates`)) (`self.bCharacterOperates`)) (`self.bUnlocked`))
          (set `self.New Open Amount` 1.0)
          (return false)
          (else
            (return false)))))
    (:`CastFailed`
      (return false))))

(fn `Reset`
  (bind _returnvalue (`KismetTextLibrary.Conv_NameToText` (`self.Input Channel`)))
  (set `self.Open Amount` (`self.New Open Amount`))
  (`self.AdjustDoorOpenness`)
  (`/Game/Robot_Dynamite/Effects/Communication/BP_TransceiverComponent.Tune In Float` (`self.BP_Transceiver`) (`self.Input Channel`))
  (`/Game/Robot_Dynamite/Effects/Communication/BP_TransceiverComponent.Tune In Float` (`self.BP_Transceiver`) (`self.Unlock Channel`))
  (`TextRenderComponent.K2_SetText` (`self.In Channel Text`) _returnvalue)
  (`TextRenderComponent.K2_SetText` (`self.In Channel Text Other Side`) _returnvalue))

(fn `UserConstructionScript`
  (`self.Reset`))