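; Actor component that lets its owner send and receive integer and float values on channels.
; Every call forwards to BP_GameState, which acts as the central channel hub.
; Tune-in functions register the owning actor on a channel, and BeginPlay tunes it into every channel in its AutoTuneInInteger and AutoTuneInFloat lists.
; Receive functions return the value along with whether the channel exists.
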(event `self.ReceiveBeginPlay`
  (for _array_element (`self.Auto Tune In Integer`)
    (`self.Tune In Integer` _array_element))
  (for _array_element_2 (`self.Auto Tune In Float`)
    (`self.Tune In Float` _array_element_2)))

(fn `Receive Float`
  (params (Channel :type Name))
  (returns (Value :type "Float (double-precision)") (`Channel Exists` :type Boolean))
  (bind (_value _channel_exists) (`/Game/Robot_Dynamite/Base/GameFramework/BP_GameState.Receive Float` (cast `/Game/Robot_Dynamite/Base/GameFramework/BP_GameState` (`GameplayStatics.GetGameState`) :!pure true) Channel))
  (return _value _channel_exists))

(fn `Receive Integer`
  (params (Channel :type Name))
  (returns (Value :type Integer) (`Channel Exists` :type Boolean))
  (bind (_value _channel_exists) (`/Game/Robot_Dynamite/Base/GameFramework/BP_GameState.Receive Integer` (cast `/Game/Robot_Dynamite/Base/GameFramework/BP_GameState` (`GameplayStatics.GetGameState`) :!pure true) Channel))
  (return _value _channel_exists))

(fn `Send Float`
  (params (Channel :type Name) (Value :type "Float (double-precision)"))
  (`/Game/Robot_Dynamite/Base/GameFramework/BP_GameState.Send Float` (cast `/Game/Robot_Dynamite/Base/GameFramework/BP_GameState` (`GameplayStatics.GetGameState`) :!pure true) Channel Value)
  (return))

(fn `Send Integer`
  (params (Channel :type Name) (Value :type Integer))
  (`/Game/Robot_Dynamite/Base/GameFramework/BP_GameState.Send Integer` (cast `/Game/Robot_Dynamite/Base/GameFramework/BP_GameState` (`GameplayStatics.GetGameState`) :!pure true) Channel Value)
  (return))

(fn `Tune In Float`
  (params (Channel :type Name))
  (`/Game/Robot_Dynamite/Base/GameFramework/BP_GameState.Tune In Float` (cast `/Game/Robot_Dynamite/Base/GameFramework/BP_GameState` (`GameplayStatics.GetGameState`) :!pure true) Channel (`self.GetOwner`))
  (return))

(fn `Tune In Integer`
  (params (Channel :type Name))
  (`/Game/Robot_Dynamite/Base/GameFramework/BP_GameState.Tune In Integer` (cast `/Game/Robot_Dynamite/Base/GameFramework/BP_GameState` (`GameplayStatics.GetGameState`) :!pure true) Channel (`self.GetOwner`))
  (return))