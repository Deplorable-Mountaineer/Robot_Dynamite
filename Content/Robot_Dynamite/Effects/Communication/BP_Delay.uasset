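; BP_Delay is a signal relay that forwards float values between transceiver channels after a configurable delay.
; On BeginPlay its BPTransceiver tunes to the input channel, and received values on an existing channel go out on the output channel after the wait.
; It uses a single latent Delay, so values arriving during the wait are not queued.
; The construction script displays the delay time on a text component.
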(event `self.ReceiveBeginPlay`
  (`/Game/Robot_Dynamite/Effects/Communication/BP_TransceiverComponent.Tune In Float` (`self.BP_Transceiver`) (`self.Input Channel`)))

(event `self.BP_Transceiver.Float Received`
  (bind (_value _channel_exists) (`/Game/Robot_Dynamite/Effects/Communication/BP_TransceiverComponent.Receive Float` (`self.BP_Transceiver`) (`self.Input Channel`)))
  (if _channel_exists
    (`KismetSystemLibrary.Delay` (`self.Delay`))
    (`/Game/Robot_Dynamite/Effects/Communication/BP_TransceiverComponent.Send Float` (`self.BP_Transceiver`) (`self.Output Channel`) _value)))

(fn `UserConstructionScript`
  (`TextRenderComponent.K2_SetText` (`self.DelayText`) (`KismetTextLibrary.Conv_DoubleToText` (`self.Delay`) "HalfFromZero" true 1 324 0 1)))