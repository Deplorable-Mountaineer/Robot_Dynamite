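; Generic switch actor that holds a float position and broadcasts it on an output transceiver channel.
; Input-channel values, permitted Operate calls or overlaps, optional retriggerable auto timers and continuous adjustment drive the position.
; SetPosition clamps or circularly wraps it, then passes it through ConvertPosition, a pass-through hook, and calls an empty OnStateChange event.
; Construction adds hidden-in-game placeholder switch meshes when no mesh exists and labels the output channel.
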(event `self.ReceiveBeginPlay`
  (`self.Reset`))

(event `self.BP_Transceiver.Float Received`
  (bind (_value _channel_exists) (`/Game/Robot_Dynamite/Effects/Communication/BP_TransceiverComponent.Receive Float` (`self.BP_Transceiver`) (`self.Channel In`)))
  (if _channel_exists
    (`self.Set Position` _value)))

(event `On State Change`
  (params (Position :type "Float (double-precision)" :default 0.0)))

(event `Next`
  (bind _position (`self.Get Position`))
  (bind _advance_amount (`self.Advance Amount`))
  ;[1 1 1] Adjustments
  (`/Game/Robot_Dynamite/Base/BPML_Utilities_Actors.Debug` false "Old:" (`KismetStringLibrary.Conv_DoubleToString` _position) "New:" (`KismetStringLibrary.Conv_DoubleToString` _advance_amount))
  (`self.Set Position` (+ _position _advance_amount)))

(event `Previous`
  ;[1 1 1] Adjustments
  (`self.Set Position` (- (`self.Get Position`) (`self.Advance Amount`))))

(event `Full On`
  ;[1 1 1] Adjustments
  (`self.Set Position` (`self.Max`)))

(event `Full Off`
  ;[1 1 1] Adjustments
  (`self.Set Position` (`self.Min`)))

(event `self.ReceiveTick`
  (params (DeltaSeconds :type "Float (single-precision)"))
  (bind _autonext (`self.AutoNext`))
  (bind _autoprevious (`self.AutoPrevious`))
  (bind _autofullon (`self.AutoFullOn`))
  (bind _autofulloff (`self.AutoFullOff`))
  (bind _autoadjustcontinuous (`self.AutoAdjustContinuous`))
  (if (`self.bStateChanged`)
    (set `self.bStateChanged` false)
    (`|ExecutionSequence`
      (:`then_0`
        (if (not (== _autonext 0.0))
          (`KismetSystemLibrary.RetriggerableDelay` _autonext)
          (`self.Next`)))
      (:`then_1`
        (if (not (== _autoprevious 0.0))
          (`KismetSystemLibrary.RetriggerableDelay` _autoprevious)
          (`self.Previous`)))
      (:`then_2`
        (if (not (== _autofullon 0.0))
          (`KismetSystemLibrary.RetriggerableDelay` _autofullon)
          (`self.Full On`)))
      (:`then_3`
        (if (not (== _autofulloff 0.0))
          (`KismetSystemLibrary.RetriggerableDelay` _autofulloff)
          (`self.Full Off`)))
      (:`then_4`
        (if (not (== _autoadjustcontinuous 0.0)) :!label _label
          (`self.Set Position` (+ (* _autoadjustcontinuous DeltaSeconds) (`self.Get Position`))))))
    (else
      (goto _label))))

(event `self.ReceiveActorBeginOverlap`
  (params (OtherActor :type "Actor Object Reference"))
  (`/Game/Robot_Dynamite/Base/BPML_Utilities_Actors.Debug` false "Overlap")
  (bind _asbp_character (cast `/Game/Robot_Dynamite/Characters/BP_Character` OtherActor))
  (if (or (and (`Pawn.IsPlayerControlled` _asbp_character) (`self.bPlayerOverlaps`)) (`self.bCharacterOverlaps`))
    (`self.Next`)))

(fn `ConvertPosition`
  (params (In :type "Float (double-precision)"))
  (returns (Out :type "Float (double-precision)"))
  (return In))

(fn `Filter Position`
  (params (In :type "Float (double-precision)"))
  (returns (Out :type "Float (double-precision)"))
  (bind _returnvalue (- (+ (`self.Max`) (`self.Advance Amount`)) (`self.Min`)))
  (if (`self.bCircular`)
    (return (+ (mod (+ (mod (- In (`self.Min`)) _returnvalue) _returnvalue) _returnvalue) (`self.Min`)))
    (else
      (return (`KismetMathLibrary.FClamp` In (`self.Min`) (`self.Max`))))))

(fn `Get Position`
  (returns (Position :type "Float (double-precision)"))
  (return (`self.Position`)))

(fn `Operate`
  (params (Operator :type "/Game/Robot_Dynamite/Characters/BP_Character Object Reference"))
  (returns (Success :type Boolean))
  (if (or (and (`Pawn.IsPlayerControlled` Operator) (`self.bPlayerOperates`)) (`self.bCharacterOperates`))
    (`/Game/Robot_Dynamite/Base/BPML_Utilities_Actors.Debug` false "Operate")
    (`self.Next`)
    (return true)
    (else
      (return false))))

(fn `Reset`
  (bind _out (`self.ConvertPosition` (`self.Filter Position` (`self.StartPosition`))))
  (`self.Set Switch State` _out)
  (`/Game/Robot_Dynamite/Effects/Communication/BP_TransceiverComponent.Tune In Float` (`self.BP_Transceiver`) (`self.Channel In`))
  (`/Game/Robot_Dynamite/Effects/Communication/BP_TransceiverComponent.Send Float` (`self.BP_Transceiver`) (`self.Channel Out`) _out))

(fn `Set Position`
  (params (Position :type "Float (double-precision)"))
  (bind _out (`self.ConvertPosition` (`self.Filter Position` Position)))
  (`self.Set Switch State` _out)
  (`/Game/Robot_Dynamite/Effects/Communication/BP_TransceiverComponent.Send Float` (`self.BP_Transceiver`) (`self.Channel Out`) _out)
  (`/Game/Robot_Dynamite/Base/BPML_Utilities_Actors.Debug` false "Send float:" (`KismetStringLibrary.Conv_DoubleToString` _out)))

(fn `Set Switch State`
  (params (Position :type "Float (double-precision)"))
  (set `self.bStateChanged` (!= Position (`self.Position`)))
  (bind _output_get (set `self.Position` Position))
  (`self.On State Change` _output_get)
  (return))

(fn `UserConstructionScript`
  (if (not (> (`KismetArrayLibrary.Array_Length` (`self.K2_GetComponentsByClass` "/Script/Engine.MeshComponent")) 0))
    (bind _returnvalue (`AddComponent|NODE_AddStaticMeshComponent-0` :`bManualAttachment` true :`RelativeTransform` (`KismetMathLibrary.MakeTransform` (0.0 0.0 10.0) (struct :`Yaw` -90.0 :`Roll` -90.0))))
    (`SceneComponent.K2_AttachToComponent` _returnvalue (`self.DefaultSceneRoot`) "None" "KeepRelative" "KeepRelative" "KeepRelative" true)
    (`StaticMeshComponent.SetStaticMesh` _returnvalue "/Game/Robot_Dynamite/Effects/Switches/SM_Switch_Multi.SM_Switch_Multi")
    (`SceneComponent.SetHiddenInGame` _returnvalue true false)
    (bind _returnvalue_2 (`AddComponent|NODE_AddStaticMeshComponent-1` :`bManualAttachment` true :`RelativeTransform` (`KismetMathLibrary.MakeTransform` (0.0 0.0 0.0))))
    (`SceneComponent.K2_AttachToComponent` _returnvalue_2 _returnvalue "NeutralPosition" "KeepRelative" "KeepRelative" "KeepRelative" true)
    (`StaticMeshComponent.SetStaticMesh` _returnvalue_2 "/Game/Robot_Dynamite/Effects/Switches/SM_Switch_Multi_Toggle.SM_Switch_Multi_Toggle")
    (`SceneComponent.SetHiddenInGame` _returnvalue_2 true false))
  (`TextRenderComponent.K2_SetText` (`self.Out Channel Text`) (`KismetTextLibrary.Conv_NameToText` (`self.Channel Out`)))
  (bind _out (`self.ConvertPosition` (`self.Filter Position` (`self.StartPosition`))))
  (`self.Set Switch State` _out)
  (set `self.StartPosition` _out))