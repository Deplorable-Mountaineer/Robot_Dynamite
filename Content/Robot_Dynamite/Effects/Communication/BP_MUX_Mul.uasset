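; BP_MUX_Mul is a multiplying multiplexer for channel-based communication, overriding only construction and the Combiner function of its parent.
; Combiner folds all input values into one product through an accumulator.
; The construction script re-targets one LCD component at three material slots on EditorMesh, rendering the input channel list, a "PRODUCT" label and the output channel as orange text.
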(fn `Combiner`
  (params (Inputs :type "Array of Float (double-precision) (by ref)"))
  (returns (Output :type "Float (double-precision)"))
  (locals (Accumulator :type "Float (double-precision)" :default 1.0))
  (for _array_element Inputs
    (set `local.Accumulator` (* _array_element (`local.Accumulator`))))
  (return (`local.Accumulator`)))

(fn `UserConstructionScript`
  (locals (`Input Channel Text` :type Text))
  (bind _lcd_inputs (`self.LCD_Inputs`))
  (bind _lcd_inputs_2 (`self.LCD_Inputs`))
  (bind _lcd_inputs_3 (`self.LCD_Inputs`))
  (`parent.UserConstructionScript`)
  (`|ExecutionSequence`
    (:`then_0`
      (set `/Game/Robot_Dynamite/Effects/LCD/BP_LCD_Component.LCD Mesh Component` (`self.EditorMesh`) _lcd_inputs_3)
      (set `/Game/Robot_Dynamite/Effects/LCD/BP_LCD_Component.LCD Material Index` 1 _lcd_inputs_3)
      (`/Game/Robot_Dynamite/Effects/LCD/BP_LCD_Component.Init` _lcd_inputs_3)
      (for _array_element (`self.Input Channels`)
        (set `local.Input Channel Text` (`|FormatText` "{0} \n{1}" (`local.Input Channel Text`) (`KismetTextLibrary.Conv_NameToText` _array_element))))
      (`/Game/Robot_Dynamite/Effects/LCD/BP_LCD_Component.SetRenderTextureParameters` _lcd_inputs_3 (`local.Input Channel Text`) (struct :`R` 1.0 :`G` 0.278321 :`A` 1.0) 1.0))
    (:`then_1`
      (set `/Game/Robot_Dynamite/Effects/LCD/BP_LCD_Component.LCD Mesh Component` (`self.EditorMesh`) _lcd_inputs)
      (set `/Game/Robot_Dynamite/Effects/LCD/BP_LCD_Component.LCD Material Index` 6 _lcd_inputs)
      (`/Game/Robot_Dynamite/Effects/LCD/BP_LCD_Component.Init` _lcd_inputs)
      (`/Game/Robot_Dynamite/Effects/LCD/BP_LCD_Component.SetRenderTextureParameters` _lcd_inputs "  PRODUCT" (struct :`R` 1.0 :`G` 0.278321 :`A` 1.0) 2.6))
    (:`then_2`
      (set `/Game/Robot_Dynamite/Effects/LCD/BP_LCD_Component.LCD Mesh Component` (`self.EditorMesh`) _lcd_inputs_2)
      (set `/Game/Robot_Dynamite/Effects/LCD/BP_LCD_Component.LCD Material Index` 7 _lcd_inputs_2)
      (`/Game/Robot_Dynamite/Effects/LCD/BP_LCD_Component.Init` _lcd_inputs_2)
      (`/Game/Robot_Dynamite/Effects/LCD/BP_LCD_Component.SetRenderTextureParameters` _lcd_inputs_2 (`KismetTextLibrary.Conv_NameToText` (`self.Output Channel`)) (struct :`R` 1.0 :`G` 0.278321 :`A` 1.0) 1.0))))