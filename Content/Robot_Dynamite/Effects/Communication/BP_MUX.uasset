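; BP_MUX is a signal combiner that merges several float channels into one output channel through a transceiver component.
; On BeginPlay it tunes the transceiver to every input channel.
; Whenever a float arrives, it re-reads all inputs, sums them in Combiner and sends the total on the output channel, so it adds signals rather than selecting one.
; The construction script shows the output channel on a text label.
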(event `self.ReceiveBeginPlay`
  (for _array_element (`self.Input Channels`)
    (`/Game/Robot_Dynamite/Effects/Communication/BP_TransceiverComponent.Tune In Float` (`self.BP_Transceiver`) _array_element)))

(event `self.BP_Transceiver.Float Received`
  (`KismetArrayLibrary.Array_Clear` (`self.Inputs`))
  (for _array_element (`self.Input Channels`)
    (bind _value (`/Game/Robot_Dynamite/Effects/Communication/BP_TransceiverComponent.Receive Float` (`self.BP_Transceiver`) _array_element))
    (`KismetArrayLibrary.Array_Add` (`self.Inputs`) _value))
  (bind _output (`self.Combiner` (`self.Inputs`)))
  (`/Game/Robot_Dynamite/Effects/Communication/BP_TransceiverComponent.Send Float` (`self.BP_Transceiver`) (`self.Output Channel`) _output)
  (`/Game/Robot_Dynamite/Base/BPML_Utilities_Actors.Debug` false "Sending:" (`KismetStringLibrary.Conv_DoubleToString` _output)))

(fn `Combiner`
  (params (Inputs :type "Array of Float (double-precision)"))
  (returns (Output :type "Float (double-precision)"))
  (locals (Accumulator :type "Float (double-precision)"))
  (bind _accumulator (`local.Accumulator`))
  (for _array_element Inputs
    (set `local.Accumulator` (+ _array_element _accumulator)))
  (return _accumulator))

(fn `UserConstructionScript`
  (`TextRenderComponent.K2_SetText` (`self.OutChannelText`) (`KismetTextLibrary.Conv_NameToText` (`self.Output Channel`))))