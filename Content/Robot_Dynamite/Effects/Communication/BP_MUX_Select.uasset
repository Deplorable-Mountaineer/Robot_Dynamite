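; BP_MUX_Select is a multiplexer in the communication effects set that passes one of several inputs through, chosen by a received channel value.
; On BeginPlay its transceiver tunes in to a float on SelectChannel, and each received value is stored as SelectedInput.
; The Combiner function rounds that value, clamps it to the valid index range and returns the matching input.
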(event `self.ReceiveBeginPlay`
  (`parent.ReceiveBeginPlay`)
  (`/Game/Robot_Dynamite/Effects/Communication/BP_TransceiverComponent.Tune In Float` (`self.BP_Transceiver`) (`self.Select Channel`)))

(event `self.BP_Transceiver.Float Received`
  (bind _value (`/Game/Robot_Dynamite/Effects/Communication/BP_TransceiverComponent.Receive Float` (`self.BP_Transceiver`) (`self.Select Channel`)))
  (bind _output_get (set `self.Selected Input` _value))
  (`/Game/Robot_Dynamite/Base/BPML_Utilities_Actors.Debug` false "Receiving:" (`KismetStringLibrary.Conv_DoubleToString` _output_get)))

(fn `Combiner`
  (params (Inputs :type "Array of Float (double-precision) (by ref)"))
  (returns (Output :type "Float (double-precision)"))
  (return (`|GetArrayItem` Inputs (`KismetMathLibrary.Clamp` (`KismetMathLibrary.Round` (`self.Selected Input`)) 0 (- (`KismetArrayLibrary.Array_Length` Inputs) 1)))))

(fn `UserConstructionScript`
  (`parent.UserConstructionScript`))