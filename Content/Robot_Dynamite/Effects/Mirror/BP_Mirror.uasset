(event `self.Collider.OnComponentBeginOverlap`
  (params (OverlappedComponent :type "PrimitiveComponent Object Reference") (OtherActor :type "Actor Object Reference") (OtherComp :type "PrimitiveComponent Object Reference") (OtherBodyIndex :type Integer) (bFromSweep :type Boolean) (SweepResult :type "HitResult Structure (by ref)"))
  (cast `/Game/Robot_Dynamite/Characters/Player/BP_RobotDynamite` OtherActor)
  (set `self.bPlayerOverlaps` true))

(event `self.Collider.OnComponentEndOverlap`
  (params (OverlappedComponent :type "PrimitiveComponent Object Reference") (OtherActor :type "Actor Object Reference") (OtherComp :type "PrimitiveComponent Object Reference") (OtherBodyIndex :type Integer))
  (cast `/Game/Robot_Dynamite/Characters/Player/BP_RobotDynamite` OtherActor)
  (set `self.bPlayerOverlaps` false))

(event `self.ReceiveBeginPlay`
  (bind _mirror (`self.Mirror`))
  (bind _asbp_robot_dynamite (cast `/Game/Robot_Dynamite/Characters/Player/BP_RobotDynamite` (`GameplayStatics.GetPlayerPawn` 0)))
  (add `/Game/Robot_Dynamite/Characters/Player/BP_RobotDynamite.Operate` _asbp_robot_dynamite (delegate `Operate`))
  (bind _returnvalue (`KismetRenderingLibrary.CreateRenderTarget2D` 512 512))
  (bind _returnvalue_2 (`PrimitiveComponent.CreateDynamicMaterialInstance` _mirror 0 (`PrimitiveComponent.GetMaterial` _mirror 0)))
  (`MaterialInstanceDynamic.SetTextureParameterValue` _returnvalue_2 "RenderTexture" _returnvalue)
  (set `SceneCaptureComponent2D.TextureTarget` _returnvalue (`self.NewSceneCaptureComponent2D`)))

(event `Operate`
  (if (and (`self.bPlayerOverlaps`) (not (`self.bUsed`)))
    (`/Game/Robot_Dynamite/Base/BPML_Utilities.RobotDynamiteSay` "You talkin' to me?" "/Game/Robot_Dynamite/Sound/PickupSound.PickupSound")
    (set `self.bUsed` true)))

(fn `UserConstructionScript`)