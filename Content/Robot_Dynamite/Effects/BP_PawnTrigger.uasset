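; BP_PawnTrigger is a trigger volume that switches tagged actors when something, optionally only a Player-tagged actor, overlaps it.
; Entering always fires it, and leaving also fires when TriggerWhenLeaving is set.
; It finds actors by Tag and calls On or Off through BPI_Switchable according to EOnTrigger.
; Toggle uses one FlipFlop inside the loop, so it alternates per actor rather than per trigger.
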(event `self.TriggerCollider.OnComponentEndOverlap`
  (params (OverlappedComponent :type "PrimitiveComponent Object Reference") (OtherActor :type "Actor Object Reference") (OtherComp :type "PrimitiveComponent Object Reference") (OtherBodyIndex :type Integer))
  (if (`self.bTriggerWhenLeaving`)
    (if (or (`self.ActorHasTag` (stale `self.TriggerCollider.OnComponentBeginOverlap` OtherActor) "Player") (not (`self.bPlayerOnly`))) :!label _label
      (bind _outactors (`GameplayStatics.GetAllActorsWithTag` (`self.Tag`)))
      (for _array_element _outactors
        (bind _asbpi_switchable (cast `/Game/Robot_Dynamite/Base/BPI_Switchable` _array_element))
        (switch `/Game/Robot_Dynamite/Effects/E_SwitchTrigger` (`self.eOnTrigger`)
          (:`NewEnumerator0`
            (`/Game/Robot_Dynamite/Base/BPI_Switchable.On` _asbpi_switchable :!label _label_2))
          (:`NewEnumerator1`
            (`/Game/Robot_Dynamite/Base/BPI_Switchable.Off` _asbpi_switchable :!label _label_3))
          (:`NewEnumerator2`
            (`/Engine/EditorBlueprintResources/StandardMacros.FlipFlop`
              (:`A`
                (goto _label_2))
              (:`B`
                (goto _label_3)))))))))

(event `self.TriggerCollider.OnComponentBeginOverlap`
  (params (OverlappedComponent :type "PrimitiveComponent Object Reference") (OtherActor :type "Actor Object Reference") (OtherComp :type "PrimitiveComponent Object Reference") (OtherBodyIndex :type Integer) (bFromSweep :type Boolean) (SweepResult :type "HitResult Structure (by ref)"))
  (goto _label))

(fn `UserConstructionScript`)