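; A mirror interactable in the Robot Dynamite game that gives the player's robot a one-time quip.
; A collider tracks whether BP_RobotDynamite overlaps it.
; On BeginPlay it binds to the player pawn's Operate event, and when operated while overlapped and unused it calls RobotDynamiteSay with a line and sound, then marks itself used.
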(event `self.Collider.OnComponentBeginOverlap`
  (params (OverlappedComponent :type "PrimitiveComponent Object Reference") (OtherActor :type "Actor Object Reference") (OtherComp :type "PrimitiveComponent Object Reference") (OtherBodyIndex :type Integer) (bFromSweep :type Boolean) (SweepResult :type "HitResult Structure (by ref)"))
  (cast `/Game/Robot_Dynamite/Characters/Player/BP_RobotDynamite` OtherActor)
  (set `self.bPlayerOverlaps` true))

(event `self.Collider.OnComponentEndOverlap`
  (params (OverlappedComponent :type "PrimitiveComponent Object Reference") (OtherActor :type "Actor Object Reference") (OtherComp :type "PrimitiveComponent Object Reference") (OtherBodyIndex :type Integer))
  (cast `/Game/Robot_Dynamite/Characters/Player/BP_RobotDynamite` OtherActor)
  (set `self.bPlayerOverlaps` false))

(event `self.ReceiveBeginPlay`
  (bind _asbp_robot_dynamite (cast `/Game/Robot_Dynamite/Characters/Player/BP_RobotDynamite` (`GameplayStatics.GetPlayerPawn` 0)))
  (add `/Game/Robot_Dynamite/Characters/Player/BP_RobotDynamite.Operate` _asbp_robot_dynamite (delegate `Operate`)))

(event `Operate`
  (if (and (`self.bPlayerOverlaps`) (not (`self.bUsed`)))
    (`/Game/Robot_Dynamite/Base/BPML_Utilities.RobotDynamiteSay` "You talkin' to me?" "/Game/Robot_Dynamite/Sound/PickupSound.PickupSound")
    (set `self.bUsed` true)))

(fn `UserConstructionScript`)