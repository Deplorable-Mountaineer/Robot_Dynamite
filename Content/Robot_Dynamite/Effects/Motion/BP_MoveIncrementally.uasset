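; Motion effect that moves itself one waypoint at a time, forward on On/Next and back on Off/Previous.
; Each request is accepted only once the current move completes, then stores start and target transforms, with the waypoint index either looping or clamping at the ends.
; Tick linearly blends the full world transform over TimeToGoal, without sweeping.
; BeginPlay sets the index to the first waypoint if already positioned there.
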(event `self.ReceiveBeginPlay`
  (`self.Init`))

(event `/Game/Robot_Dynamite/Base/BPI_Switchable.On`
  (bind _waypoints (`self.Waypoints`))
  (if (and (>= (`self.CurrentProgress`) 1.0) (> (`KismetArrayLibrary.Array_Length` _waypoints) 0)) :!label _label
    (`self.IncrementCurrentWaypoint`)
    (set `self.PreviousTransform` (`self.K2_GetComponentToWorld`))
    (set `self.CurrentTransform` (`self.K2_GetComponentToWorld` (`/Game/Robot_Dynamite/Effects/Motion/BP_Waypoint.DefaultSceneRoot` (`|GetArrayItem` _waypoints (`self.CurrentWaypoint`)))))
    (set `self.CurrentProgress` 0.0)))

(event `Next`
  (goto _label))

(event `/Game/Robot_Dynamite/Base/BPI_Switchable.Off`
  (bind _waypoints (`self.Waypoints`))
  (if (and (>= (`self.CurrentProgress`) 1.0) (> (`KismetArrayLibrary.Array_Length` _waypoints) 0)) :!label _label_2
    (if (< (`self.CurrentWaypoint`) 0)
      (set `self.CurrentWaypoint` 0))
    (`self.DecrementCurrentWaypoint`)
    (set `self.PreviousTransform` (`self.K2_GetComponentToWorld`))
    (set `self.CurrentTransform` (`self.K2_GetComponentToWorld` (`/Game/Robot_Dynamite/Effects/Motion/BP_Waypoint.DefaultSceneRoot` (`|GetArrayItem` _waypoints (`self.CurrentWaypoint`)))))
    (set `self.CurrentProgress` 0.0)))

(event `Previous`
  (goto _label_2))

(event `self.ReceiveTick`
  (params (DeltaSeconds :type "Float (single-precision)"))
  (set `self.CurrentProgress` (`KismetMathLibrary.FClamp` (+ (/ DeltaSeconds (`self.TimeToGoal`)) (`self.CurrentProgress`))))
  (`self.K2_SetWorldTransform` (`KismetMathLibrary.TLerp` (`self.PreviousTransform`) (`self.CurrentTransform`) (`self.CurrentProgress`))))

(fn `DecrementCurrentWaypoint`
  (bind _currentwaypoint (`self.CurrentWaypoint`))
  (bind _returnvalue (`KismetArrayLibrary.Array_Length` (`self.Waypoints`)))
  (set `self.CurrentWaypoint` (select `bool` (`self.bLoop`) :`false` (`KismetMathLibrary.Max` (- _currentwaypoint 1)) :`true` (mod (+ _currentwaypoint (- _returnvalue 1)) _returnvalue)))
  (return))

(fn `IncrementCurrentWaypoint`
  (bind _returnvalue (`KismetArrayLibrary.Array_Length` (`self.Waypoints`)))
  (bind _returnvalue_2 (+ (`self.CurrentWaypoint`) 1))
  (set `self.CurrentWaypoint` (select `bool` (`self.bLoop`) :`false` (`KismetMathLibrary.Min` _returnvalue_2 (- _returnvalue 1)) :`true` (mod _returnvalue_2 _returnvalue)))
  (return))

(fn `Init`
  (bind _returnvalue (`self.K2_GetComponentToWorld`))
  (bind _waypoints (`self.Waypoints`))
  (set `self.CurrentTransform` _returnvalue)
  (set `self.PreviousTransform` _returnvalue)
  (if (> (`KismetArrayLibrary.Array_Length` _waypoints) 0)
    (if (`KismetMathLibrary.NearlyEqual_TransformTransform` _returnvalue (`self.K2_GetComponentToWorld` (`/Game/Robot_Dynamite/Effects/Motion/BP_Waypoint.DefaultSceneRoot` (`|GetArrayItem` _waypoints))))
      (set `self.CurrentWaypoint` 0))))