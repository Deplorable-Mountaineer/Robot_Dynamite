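; BP_Fall is a motion effect, apparently a scene component, that makes itself fall at a constant speed until it rests on static world geometry.
; Each tick it traces along its negative up vector over that frame's FallRate-scaled step, against WorldStatic objects only.
; It snaps to the impact point on a hit, otherwise moves the full step, without sweeping or acceleration.
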(event `self.ReceiveTick`
  (params (DeltaSeconds :type "Float (single-precision)"))
  (bind _returnvalue (`self.K2_GetComponentLocation`))
  (bind _returnvalue_2 (- _returnvalue (* (`self.GetUpVector`) (* DeltaSeconds (`self.FallRate`)))))
  (bind (_outhit _returnvalue_3) (`KismetSystemLibrary.LineTraceSingleForObjects` _returnvalue _returnvalue_2 (`|MakeArray` "ObjectTypeQuery1" :!type "EObjectTypeQuery Enum")))
  (if _returnvalue_3
    (`self.K2_SetWorldLocation` (`.ImpactPoint` (`GameplayStatics.BreakHitResult` _outhit)))
    (else
      (`self.K2_SetWorldLocation` _returnvalue_2))))