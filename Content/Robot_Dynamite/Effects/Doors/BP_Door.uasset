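; BP_Door is a door Blueprint that tracks an open or closed state and opens automatically when its Trigger is overlapped.
; Open and Close events only set the Open flag, with no door movement in these graphs.
; While open with a positive AutoCloseDelay, Tick runs a Delay, then closes the door unless a Pawn still overlaps the Trigger.
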(event `Open`
  (set `self.bOpen` true))

(event `Close`
  (set `self.bOpen` false))

(event `self.Trigger.OnComponentBeginOverlap`
  (params (OverlappedComponent :type "PrimitiveComponent Object Reference") (OtherActor :type "Actor Object Reference") (OtherComp :type "PrimitiveComponent Object Reference") (OtherBodyIndex :type Integer) (bFromSweep :type Boolean) (SweepResult :type "HitResult Structure (by ref)"))
  (`self.AutoOpen`))

(event `AutoOpen`
  (if (not (`self.bOpen`))
    (`self.Open`)))

(event `self.ReceiveTick`
  (params (DeltaSeconds :type "Float (single-precision)"))
  (if (and (> (`self.Auto Close Delay`) 0.0) (`self.bOpen`))
    (`KismetSystemLibrary.Delay` (`self.Auto Close Delay`))
    (if (not (and (> (`KismetArrayLibrary.Array_Length` (`PrimitiveComponent.GetOverlappingActors` (`self.Trigger`) "/Script/Engine.Pawn")) 0) (`self.bOpen`)))
      (`self.Close`))))

(fn `UserConstructionScript`)