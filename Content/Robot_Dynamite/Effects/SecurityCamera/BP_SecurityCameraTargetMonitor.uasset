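; Monitor actor that displays the feed of a linked security camera on its screen mesh.
; At construction it registers itself with the assigned SecurityCamera, if that reference is valid.
; SetRenderTarget creates a dynamic material instance for the Monitor's screen material slot and feeds the given render target into its RenderTexture parameter.
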(fn `SetRenderTarget`
  (params (RenderTarget :type "TextureRenderTarget2D Object Reference"))
  (bind _monitor (`self.Monitor`))
  (bind _returnvalue (`KismetMaterialLibrary.CreateDynamicMaterialInstance` (`PrimitiveComponent.GetMaterial` _monitor (`self.RT_MatIndex`))))
  (`PrimitiveComponent.SetMaterial` _monitor (`self.RT_MatIndex`) _returnvalue)
  (`MaterialInstanceDynamic.SetTextureParameterValue` _returnvalue "RenderTexture" RenderTarget))

(fn `UserConstructionScript`
  (bind _securitycamera (`self.SecurityCamera`))
  (`/Engine/EditorBlueprintResources/StandardMacros.IsValid` _securitycamera
    (:`Is Valid`
      (`/Game/Robot_Dynamite/Effects/SecurityCamera/BP_SecurityCamera.RegisterMonitor` _securitycamera self))))