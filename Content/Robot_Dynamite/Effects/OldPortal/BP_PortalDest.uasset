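; Destination end of a portal that teleports overlapping actors back using its Source portal's return delta, unless return travel is blocked.
; Pawns are detached from their controller, moved and re-possessed while Source is temporarily disabled; other actors are simply moved.
; Setup creates a render target and feeds it into a dynamic M_Portal material on the Plane to display the portal view.
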(event `self.Trigger.OnComponentBeginOverlap`
  (params (OverlappedComponent :type "PrimitiveComponent Object Reference") (OtherActor :type "Actor Object Reference") (OtherComp :type "PrimitiveComponent Object Reference") (OtherBodyIndex :type Integer) (bFromSweep :type Boolean) (SweepResult :type "HitResult Structure (by ref)"))
  (bind _rootcomponent (`Actor.RootComponent` OtherActor))
  (bind _source (`self.Source`))
  (bind _result (`/Game/Robot_Dynamite/Effects/OldPortal/BP_PortalSource.AddDelta` _source (`SceneComponent.K2_GetComponentToWorld` _rootcomponent) (`/Game/Robot_Dynamite/Effects/OldPortal/BP_PortalSource.ReturnDelta` _source)))
  (if (not (or (`/Game/Robot_Dynamite/Effects/OldPortal/BP_PortalSource.bOutgoingOnly` (`self.Source`)) (`self.bDisable`)))
    (bind _aspawn (cast `Pawn` OtherActor)
      (:`then`
        (set `/Game/Robot_Dynamite/Effects/OldPortal/BP_PortalSource.bDisable` true (`self.Source`))
        (bind _output_get (set `self.PawnController` (`Pawn.GetController` _aspawn)))
        (`Pawn.DetachFromControllerPendingDestroy` _aspawn)
        (`SceneComponent.K2_SetWorldTransform` _rootcomponent _result false true)
        (`Controller.Possess` _output_get _aspawn)
        (set `/Game/Robot_Dynamite/Effects/OldPortal/BP_PortalSource.bDisable` false (`self.Source`)))
      (:`CastFailed`
        (`SceneComponent.K2_SetWorldTransform` _rootcomponent _result false true)))))

(fn `Setup`
  (bind _returnvalue (`KismetRenderingLibrary.CreateRenderTarget2D` 1920 1080))
  (set `self.RenderTarget` _returnvalue)
  (bind _returnvalue_2 (`KismetMaterialLibrary.CreateDynamicMaterialInstance` "/Game/Robot_Dynamite/Effects/OldPortal/M_Portal.M_Portal"))
  (`PrimitiveComponent.SetMaterial` (`self.Plane`) 0 _returnvalue_2)
  (`MaterialInstanceDynamic.SetTextureParameterValue` _returnvalue_2 "RenderTarget" _returnvalue))

(fn `UserConstructionScript`)