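; BP_Grenade is a grenade for the grenade launcher that explodes when the actor is destroyed.
; On Destroyed, it spawns an explosion effect actor at its transform, scaled in proportion to the inner damage radius.
; It then applies radial damage with linear falloff between inner and outer radii, down to a tenth of base damage, crediting the instigator's controller.
; The construction script only calls the parent.
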(event `self.ReceiveDestroyed`
  (bind _returnvalue (`self.GetInstigator`))
  (bind _damage (`self.Damage`))
  (bind _returnvalue_2 (`|SpawnActorFromClass` "/Game/StarterContent/Blueprints/Blueprint_Effect_Explosion.Blueprint_Effect_Explosion_C" (`self.GetTransform`) "AlwaysSpawn" "OverrideRootScale" _returnvalue _returnvalue))
  (`self.SetActorScale3D` _returnvalue_2 (`KismetMathLibrary.Conv_DoubleToVector` (/ (`self.InnerRadius`) 50.0)))
  (`GameplayStatics.ApplyRadialDamageWithFalloff` :`BaseDamage` _damage :`MinimumDamage` (/ _damage 10.0) :`Origin` (`self.K2_GetActorLocation`) :`DamageInnerRadius` (`self.InnerRadius`) :`DamageOuterRadius` (`self.OuterRadius`) :`DamageFalloff` 1.0 :`DamageCauser` self :`InstigatedByController` (`self.GetInstigatorController`)))

(fn `UserConstructionScript`
  (`parent.UserConstructionScript`))