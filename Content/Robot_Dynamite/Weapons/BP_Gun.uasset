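; Gun actor that attaches to a pawn and fires projectiles from its muzzle, hiding its mesh unless its parent is the player pawn.
; Trigger events set a flag that Tick uses to call Fire automatically, gated by ammo and a cooldown.
; Each shot spawns a projectile with the pawn as instigator, plays a sound, notifies the attach parent and spends ammo.
; Reload adds ammo, optionally ignoring the maximum.
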(event `self.ReceiveBeginPlay`
  (if (!= (`self.GetParentActor`) (`GameplayStatics.GetPlayerPawn` 0))
    (`SceneComponent.SetVisibility` (`self.SK_Gun`) false false)))

(event `self.ReceiveTick`
  (params (DeltaSeconds :type "Float (single-precision)"))
  (set `self.SecondsToFireAgain` (`KismetMathLibrary.FClamp` (- (`self.SecondsToFireAgain`) DeltaSeconds) 0.0 1000.0))
  (if (`self.bTriggerPressed`)
    (`self.Fire`)))

(event `TriggerPressed`
  (set `self.bTriggerPressed` true))

(event `TriggerReleased`
  (set `self.bTriggerPressed` false))

(fn `Fire`
  (returns (Success :type Boolean))
  (if (> (`self.AmmoAmount`) 0)
    (if (<= (`self.SecondsToFireAgain`) 0.0)
      (bind _aspawn (cast `Pawn` (`self.GetAttachParentActor`))
        (:`then`
          (`|SpawnActorFromClass` (`self.Projectile`) (`SceneComponent.K2_GetComponentToWorld` (`self.Muzzle`)) "AdjustIfPossibleButAlwaysSpawn" "OverrideRootScale" null _aspawn) ; Spawn projectile
          (`GameplayStatics.PlaySoundAtLocation` (`self.FireSound`) (`self.K2_GetActorLocation`)) ; Play firing sound
          (set `self.SecondsToFireAgain` (`self.FiringRate`))
          (message `/Game/Robot_Dynamite/Base/BPI_Character.GunFired` (`self.GetAttachParentActor`))
          (set `self.AmmoAmount` (- (`self.AmmoAmount`) 1))
          (return true))
        (:`CastFailed`
          (return false))))
    (else
      (return false))))

(fn `Reload`
  (params (Amount :type Integer) (bIgnoreMax :type Boolean))
  (returns (Success :type Boolean))
  (locals (OldAmmoAmount :type Integer))
  (bind _returnvalue (+ Amount (`self.AmmoAmount`)))
  (set `local.OldAmmoAmount` Amount)
  (bind _output_get (set `self.AmmoAmount` (select `bool` bIgnoreMax :`false` (`KismetMathLibrary.Clamp` _returnvalue 0 (`self.MaxAmmoAmount`)) :`true` _returnvalue)))
  (return (!= _output_get (`local.OldAmmoAmount`))))

(fn `UserConstructionScript`)