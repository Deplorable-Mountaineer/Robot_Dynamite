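; BP_Melee is an inventory Blueprint for a melee item that gates each use behind ammo and a cooldown.
; Fire checks the HasAmmo and ReadyToFire macros, then spends one ammo, resets SecondsToFireAgain to FiringRate and returns true, or returns false if either check fails.
; The event graph is inactive, so this file contains no cooldown countdown, hit detection or damage logic.
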(fn `Fire`
  (returns (Success :type Boolean))
  (`self.HasAmmo`
    (:`true`
      (`self.ReadyToFire`
        (:`true`
          (set `self.AmmoAmount` (- (`self.AmmoAmount`) 1.0))
          (set `self.SecondsToFireAgain` (`self.FiringRate`))
          (return true))
        (:`false`
          _)))
    (:`false`
      _))
  (return false))

(fn `UserConstructionScript`
  (`parent.UserConstructionScript`))