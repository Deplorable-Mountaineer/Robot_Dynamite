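; BP_PowerUp is an inventory power-up that tracks a consumable amount against a maximum.
; Replenish adds to the stored amount, clamped between zero and the maximum unless IgnoreMax is set, and returns whether the value changed.
; Use deducts up to what is available and returns the quantity consumed.
; Getters expose the current and maximum amounts, while the event graph and construction script hold no logic.
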(fn `GetAmount`
  (returns (Amount :type "Float (double-precision)"))
  (return (`self.Amount`)))

(fn `GetMaxAmount`
  (returns (MaxAmount :type "Float (double-precision)"))
  (return (`self.Max`)))

(fn `Replenish`
  (params (Amount :type "Float (double-precision)") (IgnoreMax :type Boolean))
  (returns (bAmountChanged :type Boolean))
  (locals (OldAmount :type "Float (double-precision)"))
  (bind _output_get (set `local.OldAmount` (`self.Amount`)))
  (bind _returnvalue (+ _output_get Amount))
  (bind _returnvalue_2 (select `bool` IgnoreMax :`false` (`KismetMathLibrary.FClamp` _returnvalue 0.0 (`self.Max`)) :`true` _returnvalue))
  (set `self.Amount` _returnvalue_2)
  (return (!= _returnvalue_2 (`local.OldAmount`))))

(fn `Use`
  (params (Amount :type "Float (double-precision)"))
  (returns (ActualAmountDeducted :type "Float (double-precision)"))
  (locals (OldAmount :type "Float (double-precision)" :default 0.0))
  (bind _output_get (set `local.OldAmount` (`self.Amount`)))
  (bind _returnvalue (`KismetMathLibrary.FMin` _output_get Amount))
  (set `self.Amount` (- _output_get _returnvalue))
  (return _returnvalue))

(fn `UserConstructionScript`)