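; Inventory component for BP_Character that builds a fixed set of slots on BeginPlay for weapons, health and armor, keys, and gear.
; Each slot is a spawned BP_Slot actor stored in a map keyed by item class, which GetSlot and GetItem look up.
; Slots flagged to spawn get their item actor immediately, attached hidden to a character mesh socket, then the character is notified through OnInventorySpawn.
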(event `self.ReceiveBeginPlay`
  (`|ExecutionSequence`
    (:`then_0`
      (`self.CreateSlot` "NewEnumerator0" "/Game/Robot_Dynamite/Inventory/BP_Melee.BP_Melee_C" true "GripPoint")
      (`self.CreateSlot` "NewEnumerator1" "/Game/Robot_Dynamite/Inventory/Weapons/Rifle/BP_Rifle.BP_Rifle_C" true "GripPoint")
      (`self.CreateSlot` "NewEnumerator1" "/Game/Robot_Dynamite/Inventory/Weapons/GrenadeLauncher/BP_GrenadeLauncher.BP_GrenadeLauncher_C" false "GripPoint"))
    (:`then_1`
      (`self.CreateSlot` "NewEnumerator3" "/Game/Robot_Dynamite/Inventory/VitalStatistics/BP_Health.BP_Health_C" true)
      (`self.CreateSlot` "NewEnumerator3" "/Game/Robot_Dynamite/Inventory/VitalStatistics/BP_Armor.BP_Armor_C" true))
    (:`then_2`
      (`self.CreateSlot` "NewEnumerator4" "/Game/Robot_Dynamite/Inventory/Keys/BP_KeyCopper.BP_KeyCopper_C")
      (`self.CreateSlot` "NewEnumerator4" "/Game/Robot_Dynamite/Inventory/Keys/BP_KeySilver.BP_KeySilver_C")
      (`self.CreateSlot` "NewEnumerator4" "/Game/Robot_Dynamite/Inventory/Keys/BP_KeyGold.BP_KeyGold_C"))
    (:`then_3`
      (`self.CreateSlot` "NewEnumerator5" "/Game/Robot_Dynamite/Inventory/PowerUps/BP_LiftBelt.BP_LiftBelt_C" false "Belt")
      (`self.CreateSlot` "NewEnumerator5" "/Game/Robot_Dynamite/Inventory/PowerUps/BP_NO2.BP_NO2_C")
      (`self.CreateSlot` "NewEnumerator5" "/Game/Robot_Dynamite/Inventory/PowerUps/BP_NVG.BP_NVG_C" false "Eyes"))))

(fn `CreateSlot`
  (params (Type :type "/Game/Robot_Dynamite/Inventory/EItemType Enum" :default "NewEnumerator0") (Class :type "/Game/Robot_Dynamite/Inventory/BP_Item Class Reference") (bSpawn :type Boolean) (Socket :type Name :default "None"))
  (returns (Slot :type "/Game/Robot_Dynamite/Inventory/BP_Slot Object Reference"))
  (bind (_class1 _slot _character _socket1) (`self.Spawn Slot` (`self.GetOwner`) Type Class Socket))
  (`BlueprintMapLibrary.Map_Add` (`self.Slots`) _class1 _slot)
  (if bSpawn
    (`self.SpawnInventoryItem` _class1 _slot _character _socket1)
    (return _slot)
    (else
      (return _slot))))

(fn `GetItem`
  (params (Key :type "Actor Class Reference"))
  (returns (Item :type "Actor Object Reference") (IsValid :type Boolean) (Slot :type "/Game/Robot_Dynamite/Inventory/BP_Slot Object Reference"))
  (bind (_value _returnvalue) (`BlueprintMapLibrary.Map_Find` (`self.Slots`) Key))
  (bind _item (`/Game/Robot_Dynamite/Inventory/BP_Slot.Item` _value))
  (if _returnvalue
    (return _item (`KismetSystemLibrary.IsValid` _item) _value)
    (else
      (`/Game/Robot_Dynamite/Base/BPML_Utilities_Components.Error` "No such slot:" (`KismetSystemLibrary.GetClassDisplayName` Key))
      (return null))))

(fn `GetSlot`
  (params (Key :type "Actor Class Reference"))
  (returns (Slot :type "/Game/Robot_Dynamite/Inventory/BP_Slot Object Reference"))
  (bind (_value _returnvalue) (`BlueprintMapLibrary.Map_Find` (`self.Slots`) Key))
  (if _returnvalue
    (return _value)
    (else
      (`/Game/Robot_Dynamite/Base/BPML_Utilities_Components.Error` "No such slot:" (`KismetSystemLibrary.GetClassDisplayName` Key))
      (return null))))

(fn `Spawn Slot`
  (params (Owner :type "Actor Object Reference") (Type :type "/Game/Robot_Dynamite/Inventory/EItemType Enum" :default "NewEnumerator1") (Class :type "/Game/Robot_Dynamite/Inventory/BP_Item Class Reference") (Socket :type Name :default "None"))
  (returns (Class1 :type "/Game/Robot_Dynamite/Inventory/BP_Item Class Reference") (Slot :type "/Game/Robot_Dynamite/Inventory/BP_Slot Object Reference") (Character :type "/Game/Robot_Dynamite/Characters/BP_Character Object Reference") (Socket1 :type Name))
  (bind _asbp_character (cast `/Game/Robot_Dynamite/Characters/BP_Character` Owner :!pure true))
  (bind _returnvalue (`|SpawnActorFromClass` "/Game/Robot_Dynamite/Inventory/BP_Slot.BP_Slot_C" (`KismetMathLibrary.MakeTransform` (0.0 0.0 0.0)) "AlwaysSpawn" "OverrideRootScale" _asbp_character Type Class Socket _asbp_character))
  (return Class _returnvalue _asbp_character Socket))

(fn `SpawnInventoryItem`
  (params (Class :type "/Game/Robot_Dynamite/Inventory/BP_Item Class Reference (by ref)") (Slot :type "/Game/Robot_Dynamite/Inventory/BP_Slot Object Reference") (Character :type "/Game/Robot_Dynamite/Characters/BP_Character Object Reference") (Socket :type Name))
  (`/Engine/EditorBlueprintResources/StandardMacros.IsValid` (`/Game/Robot_Dynamite/Inventory/BP_Slot.Item` Slot)
    (:`Is Valid`
      _)
    (:`Is Not Valid`
      (bind _returnvalue (`|SpawnActorFromClass` Class (`KismetMathLibrary.MakeTransform` (0.0 0.0 0.0)) "AlwaysSpawn" "OverrideRootScale" Character Character))
      (bind _output_get (set `/Game/Robot_Dynamite/Inventory/BP_Slot.Item` _returnvalue Slot))))
  (`Actor.K2_AttachToComponent` _output_get (`Character.Mesh` Character) Socket "KeepRelative" "KeepRelative" "KeepRelative" true)
  (`SceneComponent.SetVisibility` (`Actor.RootComponent` _output_get) false true)
  (`/Game/Robot_Dynamite/Characters/BP_Character.On Inventory Spawn` Character _output_get Socket)
  (return))