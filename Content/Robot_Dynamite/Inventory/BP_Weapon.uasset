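; Base weapon actor that fires projectiles for its owning pawn, with the gun mesh hidden unless its parent actor is the player pawn.
; While the trigger is held, Tick calls Fire, gated by ammo and a cooldown timer.
; Firing spawns a projectile at the muzzle with the pawn as instigator, plays sound, notifies the attach parent and spends one round.
; Reload adds ammo, optionally beyond maximum; Deduct is a stub.
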(event `self.ReceiveBeginPlay`
  (if (!= (`self.GetParentActor`) (`GameplayStatics.GetPlayerPawn` 0))
    (`SceneComponent.SetVisibility` (`self.SK_Gun`) false false)))

(event `self.ReceiveTick`
  (params (DeltaSeconds :type "Float (single-precision)"))
  (set `self.SecondsToFireAgain` (`KismetMathLibrary.FClamp` (- (`self.SecondsToFireAgain`) DeltaSeconds) 0.0 1000.0))
  (if (`self.bTriggerPressed`)
    (`self.Fire`)))

(event `TriggerPressed`
  (set `self.bTriggerPressed` true))

(event `TriggerReleased`
  (set `self.bTriggerPressed` false))

(fn `Deduct`
  (params (Amount :type "Float (double-precision)"))
  (returns (ActualAmountDeducted :type "Float (double-precision)"))
  (return 0.0))

(fn `Fire`
  (returns (Success :type Boolean))
  (`self.HasAmmo`
    (:`Yes`
      (`self.ReadyToFire`
        (:`Yes`
          (bind (_projectile _success) (`self.SpawnProjectile`))
          (if _success
            (`GameplayStatics.PlaySoundAtLocation` (`self.FireSound`) (`self.K2_GetActorLocation`) (struct) 1.0 (`self.FireSoundPitch`)) ; Play firing sound
            (set `self.SecondsToFireAgain` (`self.FiringRate`))
            (message `/Game/Robot_Dynamite/Base/BPI_Character.GunFired` (`self.GetAttachParentActor`))
            (set `self.AmmoAmount` (- (`self.AmmoAmount`) 1.0))
            (return true)
            (else
              (return false))))
        (:`No`
          _)))
    (:`No`
      _))
  (return false))

(fn `GetAmount`
  (returns (Amount :type "Float (double-precision)"))
  (return (`self.AmmoAmount`)))

(fn `GetMaxAmount`
  (returns (MaxAmmoAmount :type "Float (double-precision)"))
  (return (`self.MaxAmmoAmount`)))

(fn `Reload`
  (params (Amount :type "Float (double-precision)") (IgnoreMax :type Boolean))
  (returns (bAmountChanged :type Boolean))
  (locals (OldAmmoAmount :type "Float (double-precision)"))
  (bind _oldammoamount (`local.OldAmmoAmount`))
  (bind _returnvalue (+ Amount (`self.AmmoAmount`)))
  (`/Game/Robot_Dynamite/Base/BPFL_Utilities.DebugPrint` false "Reload in bp_gun")
  (set `local.OldAmmoAmount` (`self.AmmoAmount`))
  (bind _output_get (set `self.AmmoAmount` (select `bool` IgnoreMax :`false` (`KismetMathLibrary.FClamp` _returnvalue 0.0 (`self.MaxAmmoAmount`)) :`true` _returnvalue)))
  (`/Game/Robot_Dynamite/Base/BPFL_Utilities.DebugPrint` false "old/new amount" (`KismetStringLibrary.Conv_DoubleToString` _oldammoamount) (`KismetStringLibrary.Conv_DoubleToString` _output_get))
  (return (!= _output_get _oldammoamount)))

(fn `SpawnProjectile`
  (returns (Projectile :type "/Game/Robot_Dynamite/Inventory/Weapons/BP_Projectile Object Reference") (Success :type Boolean))
  (if (`KismetSystemLibrary.IsValidClass` (`self.Projectile`))
    (bind _aspawn (`self.GetPawn`)
      (:`Success`
        (bind _returnvalue (`|SpawnActorFromClass` (`self.Projectile`) (`SceneComponent.K2_GetComponentToWorld` (`self.Muzzle`)) "AdjustIfPossibleButAlwaysSpawn" "OverrideRootScale" null _aspawn)) ; Spawn projectile
        (return _returnvalue (`KismetSystemLibrary.IsValid` _returnvalue)))
      (:`Failure`
        _)))
  (return null false))

(fn `UserConstructionScript`
  (set `self.AmmoAmount` (`self.MaxAmmoAmount`)))