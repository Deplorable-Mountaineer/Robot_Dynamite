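; BP_Pickup is an item pickup that grants what it provides to a BP_Character overlapping its sphere.
; When the character accepts the item, it plays a sound, deactivates and hides itself by swapping the item mesh to an invisible one.
; With a positive respawn time, it restores the saved mesh and reactivates after that delay.
; Overlaps by other actors while active log an error.
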(event `self.Sphere.OnComponentBeginOverlap`
  (params (OverlappedComponent :type "PrimitiveComponent Object Reference") (OtherActor :type "Actor Object Reference") (OtherComp :type "PrimitiveComponent Object Reference") (OtherBodyIndex :type Integer) (bFromSweep :type Boolean) (SweepResult :type "HitResult Structure (by ref)"))
  (bind _respawntime (`self.RespawnTime`))
  (if (`self.Active`)
    (bind _asbp_character (cast `/Game/Robot_Dynamite/Characters/BP_Character` OtherActor)
      (:`then`
        (bind _success (`/Game/Robot_Dynamite/Characters/BP_Character.GetItemFromPickup` _asbp_character (`self.Provides`)))
        (if _success
          (`GameplayStatics.PlaySoundAtLocation` "/Game/Robot_Dynamite/Sound/PickupSound.PickupSound" (`self.K2_GetActorLocation` _asbp_character))
          (set `self.Active` false)
          (set `self.SaveStaticMesh` (`StaticMeshComponent.StaticMesh` (`self.Item`)))
          (`StaticMeshComponent.SetStaticMesh` (`self.Item`) "/Game/Robot_Dynamite/Environment/Props/SM_Invisible.SM_Invisible")
          (if (> _respawntime 0.0)
            (`KismetSystemLibrary.Delay` _respawntime)
            (`StaticMeshComponent.SetStaticMesh` (`self.Item`) (`self.SaveStaticMesh`))
            (set `self.Active` true))))
      (:`CastFailed`
        (`/Game/Robot_Dynamite/Base/BPML_Utilities_Actors.Error` "Not a BP_Character: " (`KismetSystemLibrary.GetDisplayName` OtherActor))))))

(fn `UserConstructionScript`)