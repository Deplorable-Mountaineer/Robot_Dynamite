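; Base level script Blueprint for Robot Dynamite that provides console cheat events invoked with "ce".
; Fly, NightVision and Run each spawn their matching item, then use a FlipFlop to toggle that ability on the player pawn.
; TakeDamage applies a given amount of damage to the player.
; Spawn creates an actor at the player from the Classes map, falling back to a closest-name match, and cheats report results through on-screen messages.
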(event `Fly`
  ;[1 1 1] ce Fly
  (`self.Spawn` "Liftbelt")
  (`/Engine/EditorBlueprintResources/StandardMacros.FlipFlop`
    (:`A`
      (bind _asbp_robot_dynamite (cast `/Game/Robot_Dynamite/Characters/Player/Robot_Dynamite/BP_RobotDynamite` (`GameplayStatics.GetPlayerPawn` 0)))
      (`/Game/Robot_Dynamite/Characters/BP_Character.StartFlying` _asbp_robot_dynamite)
      (`/Game/Robot_Dynamite/Base/BPML_Utilities_Actors.DisplayMessage` "Robot Dynamite feels very light!" (struct :`R` 0.424385 :`G` 0.040803 :`B` 0.040803 :`A` 1.0)))
    (:`B`
      (bind _asbp_robot_dynamite_2 (cast `/Game/Robot_Dynamite/Characters/Player/Robot_Dynamite/BP_RobotDynamite` (`GameplayStatics.GetPlayerPawn` 0)))
      (`/Game/Robot_Dynamite/Characters/BP_Character.StopFlying` _asbp_robot_dynamite_2)
      (`/Game/Robot_Dynamite/Base/BPML_Utilities_Actors.DisplayMessage` "Robot Dynamite feels heavy again" (struct :`R` 0.424385 :`G` 0.040803 :`B` 0.040803 :`A` 1.0)))))

(event `NightVision`
  ;[1 1 1] ce NightVision
  (`self.Spawn` "NVG")
  (`/Engine/EditorBlueprintResources/StandardMacros.FlipFlop`
    (:`A`
      (bind _asbp_robot_dynamite (cast `/Game/Robot_Dynamite/Characters/Player/Robot_Dynamite/BP_RobotDynamite` (`GameplayStatics.GetPlayerPawn` 0)))
      (`/Game/Robot_Dynamite/Characters/Player/Robot_Dynamite/BP_RobotDynamite.Start Night Vision` _asbp_robot_dynamite)
      (`/Game/Robot_Dynamite/Base/BPML_Utilities_Actors.DisplayMessage` "Robot Dynamite can see in the dark!" (struct :`R` 0.424385 :`G` 0.040803 :`B` 0.040803 :`A` 1.0)))
    (:`B`
      (bind _asbp_robot_dynamite_2 (cast `/Game/Robot_Dynamite/Characters/Player/Robot_Dynamite/BP_RobotDynamite` (`GameplayStatics.GetPlayerPawn` 0)))
      (`/Game/Robot_Dynamite/Characters/Player/Robot_Dynamite/BP_RobotDynamite.Stop Night Vision` _asbp_robot_dynamite_2)
      (`/Game/Robot_Dynamite/Base/BPML_Utilities_Actors.DisplayMessage` "Robot Dynamite has normal vision again" (struct :`R` 0.424385 :`G` 0.040803 :`B` 0.040803 :`A` 1.0)))))

(event `Run`
  ;[1 1 1] ce Run
  (`self.Spawn` "Nitro")
  (`/Engine/EditorBlueprintResources/StandardMacros.FlipFlop`
    (:`A`
      (bind _asbp_robot_dynamite (cast `/Game/Robot_Dynamite/Characters/Player/Robot_Dynamite/BP_RobotDynamite` (`GameplayStatics.GetPlayerPawn` 0)))
      (`/Game/Robot_Dynamite/Characters/BP_Character.Start Running` _asbp_robot_dynamite)
      (`/Game/Robot_Dynamite/Base/BPML_Utilities_Actors.DisplayMessage` "Robot Dynamite has a speed burst!" (struct :`R` 0.424385 :`G` 0.040803 :`B` 0.040803 :`A` 1.0)))
    (:`B`
      (bind _asbp_robot_dynamite_2 (cast `/Game/Robot_Dynamite/Characters/Player/Robot_Dynamite/BP_RobotDynamite` (`GameplayStatics.GetPlayerPawn` 0)))
      (`/Game/Robot_Dynamite/Characters/BP_Character.Stop Running` _asbp_robot_dynamite_2)
      (`/Game/Robot_Dynamite/Base/BPML_Utilities_Actors.DisplayMessage` "Robot Dynamite walks normally again" (struct :`R` 0.424385 :`G` 0.040803 :`B` 0.040803 :`A` 1.0)))))

(event `TakeDamage`
  (params (Amount :type "Float (double-precision)" :default 15.0))
  ;[1 1 1] ce TakeDamage [<amount>]
  (bind _asbp_robot_dynamite (cast `/Game/Robot_Dynamite/Characters/Player/Robot_Dynamite/BP_RobotDynamite` (`GameplayStatics.GetPlayerPawn` 0)))
  (`GameplayStatics.ApplyDamage` _asbp_robot_dynamite Amount)
  (`/Game/Robot_Dynamite/Base/BPML_Utilities_Actors.DisplayMessage` "Robot Dynamite hurt himself!" (struct :`R` 0.424385 :`G` 0.040803 :`B` 0.040803 :`A` 1.0)))

(event `Spawn`
  (params (Actor :type Name))
  (bind _returnvalue (`GameplayStatics.GetPlayerCharacter` 0))
  (bind _classes (`self.Classes`))
  (bind _returnvalue_2 (`self.GetTransform` _returnvalue))
  (bind (_value _returnvalue_3) (`BlueprintMapLibrary.Map_Find` _classes Actor))
  ;[1 1 1] ce Spawn <name>
  (if _returnvalue_3
    (bind _returnvalue_4 (`/Game/Robot_Dynamite/Base/BPML_Utilities_Actors.Spawn` _value _returnvalue_2 "AdjustIfPossibleButAlwaysSpawn" _returnvalue _returnvalue))
    (`/Game/Robot_Dynamite/Base/BPML_Utilities_Actors.DisplayMessage` (`KismetStringLibrary.Concat_StrStr` "Spawned: " (`KismetSystemLibrary.GetDisplayName` _returnvalue_4)) (struct :`R` 0.424385 :`G` 0.040803 :`B` 0.040803 :`A` 1.0))
    (else
      (bind _keys (`BlueprintMapLibrary.Map_Keys` _classes))
      (bind _match (`/Game/Robot_Dynamite/Base/BPFL_Utilities.MatchBestName` Actor _keys))
      (bind (_value_2 _returnvalue_5) (`BlueprintMapLibrary.Map_Find` (`self.Classes`) _match))
      (if _returnvalue_5
        (bind _returnvalue_6 (`/Game/Robot_Dynamite/Base/BPML_Utilities_Actors.Spawn` _value_2 _returnvalue_2 "AdjustIfPossibleButAlwaysSpawn" _returnvalue _returnvalue))
        (`/Game/Robot_Dynamite/Base/BPML_Utilities_Actors.DisplayMessage` (`KismetStringLibrary.Concat_StrStr` "Spawned: " (`KismetSystemLibrary.GetDisplayName` _returnvalue_6)) (struct :`R` 0.424385 :`G` 0.040803 :`B` 0.040803 :`A` 1.0))
        (else
          (`/Game/Robot_Dynamite/Base/BPML_Utilities_Actors.DisplayMessage` (`KismetStringLibrary.Concat_StrStr` "Failed to spawn: " (`KismetStringLibrary.Conv_NameToString` _match)) (struct :`R` 0.424385 :`G` 0.040803 :`B` 0.040803 :`A` 1.0)))))))

(fn `UserConstructionScript`)