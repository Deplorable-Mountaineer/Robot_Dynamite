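; Game state that counts enemy-tagged actors at BeginPlay and acts as a channel-based message hub for integer and float values.
; Send functions store the latest value per channel and notify BP_TransceiverComponents on that channel's registered listener actors, without passing the value.
; Tune In functions register unique listeners per channel, Receive functions return the stored value with an existence flag, and Clear Channels wipes values but keeps listeners.
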(event `self.ReceiveBeginPlay`
  (bind _outactors (`GameplayStatics.GetAllActorsWithTag` "Enemy"))
  (set `self.NumEnemies` (`KismetArrayLibrary.Array_Length` _outactors)))

(fn `Clear Channels`
  (`BlueprintMapLibrary.Map_Clear` (`self.Channels_Integer`))
  (`BlueprintMapLibrary.Map_Clear` (`self.Channels_Float`))
  (return))

(fn `Receive Float`
  (params (Channel :type Name))
  (returns (Value :type "Float (double-precision)") (`Channel Exists` :type Boolean))
  (bind (_value _returnvalue) (`BlueprintMapLibrary.Map_Find` (`self.Channels_Float`) Channel))
  (return _value _returnvalue))

(fn `Receive Integer`
  (params (Channel :type Name))
  (returns (Value :type Integer) (`Channel Exists` :type Boolean))
  (bind (_value _returnvalue) (`BlueprintMapLibrary.Map_Find` (`self.Channels_Integer`) Channel))
  (return _value _returnvalue))

(fn `Send Float`
  (params (Channel :type Name) (Value :type "Float (double-precision)"))
  (bind (_value _returnvalue) (`BlueprintMapLibrary.Map_Find` (`self.Listeners_Float`) Channel))
  (`BlueprintMapLibrary.Map_Add` (`self.Channels_Float`) Channel Value)
  (if _returnvalue
    (for _array_element (break `/Game/Robot_Dynamite/Effects/Communication/S_Listeners` _value)
      (for _array_element_2 (`self.K2_GetComponentsByClass` _array_element "/Game/Robot_Dynamite/Effects/Communication/BP_TransceiverComponent.BP_TransceiverComponent_C")
        (`/Game/Robot_Dynamite/Effects/Communication/BP_TransceiverComponent.Float Received` _array_element_2)))
    (return)
    (else
      (return))))

(fn `Send Integer`
  (params (Channel :type Name) (Value :type Integer))
  (bind (_value _returnvalue) (`BlueprintMapLibrary.Map_Find` (`self.Listeners_Integer`) Channel))
  (`BlueprintMapLibrary.Map_Add` (`self.Channels_Integer`) Channel Value)
  (if _returnvalue
    (for _array_element (break `/Game/Robot_Dynamite/Effects/Communication/S_Listeners` _value)
      (for _array_element_2 (`self.K2_GetComponentsByClass` _array_element "/Game/Robot_Dynamite/Effects/Communication/BP_TransceiverComponent.BP_TransceiverComponent_C")
        (`/Game/Robot_Dynamite/Effects/Communication/BP_TransceiverComponent.Integer Received` _array_element_2)))
    (return)
    (else
      (return))))

(fn `Tune In Float`
  (params (Channel :type Name) (Actor :type "Actor Object Reference"))
  (locals (`Current Listeners` :type "Array of Actor Object Reference"))
  (bind (_value _returnvalue) (`BlueprintMapLibrary.Map_Find` (`self.Listeners_Float`) Channel))
  (if _returnvalue
    (bind _output_get (set `local.Current Listeners` (break `/Game/Robot_Dynamite/Effects/Communication/S_Listeners` _value)))
    (else
      (`KismetArrayLibrary.Array_Clear` (`local.Current Listeners`))))
  (`KismetArrayLibrary.Array_AddUnique` (`local.Current Listeners`) Actor)
  (`BlueprintMapLibrary.Map_Add` (`self.Listeners_Float`) Channel (make `/Game/Robot_Dynamite/Effects/Communication/S_Listeners` _output_get))
  (return))

(fn `Tune In Integer`
  (params (Channel :type Name) (Actor :type "Actor Object Reference"))
  (locals (`Current Listeners` :type "Array of Actor Object Reference"))
  (bind (_value _returnvalue) (`BlueprintMapLibrary.Map_Find` (`self.Listeners_Integer`) Channel))
  (if _returnvalue
    (bind _output_get (set `local.Current Listeners` (break `/Game/Robot_Dynamite/Effects/Communication/S_Listeners` _value)))
    (else
      (`KismetArrayLibrary.Array_Clear` (`local.Current Listeners`))))
  (`KismetArrayLibrary.Array_AddUnique` (`local.Current Listeners`) Actor)
  (`BlueprintMapLibrary.Map_Add` (`self.Listeners_Integer`) Channel (make `/Game/Robot_Dynamite/Effects/Communication/S_Listeners` _output_get))
  (return))

(fn `UserConstructionScript`)