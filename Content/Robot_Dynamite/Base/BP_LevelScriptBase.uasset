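; Base level script for Robot Dynamite that provides cheat events for flying and night vision.
; Fly and Walk start or stop flying on the player's BP_RobotDynamite pawn and display a colored status message.
; NightVision and NormalVision overwrite the settings of post-process volumes tagged "NightVision", switching between a green-tinted ambient cubemap and a neutral, zero-intensity look.
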(event `Fly`
  (bind _asbp_robot_dynamite (cast `/Game/Robot_Dynamite/Characters/Player/BP_RobotDynamite` (`GameplayStatics.GetPlayerPawn` 0)))
  (`/Game/Robot_Dynamite/Characters/BP_Character.StartFlying` _asbp_robot_dynamite)
  (`/Game/Robot_Dynamite/Base/BPML_Utilities.DisplayMessage` "Robot Dynamite feels very light" (struct :`R` 0.424385 :`G` 0.040803 :`B` 0.040803 :`A` 1.0)))

(event `Walk`
  (bind _asbp_robot_dynamite (cast `/Game/Robot_Dynamite/Characters/Player/BP_RobotDynamite` (`GameplayStatics.GetPlayerPawn` 0)))
  (`/Game/Robot_Dynamite/Characters/BP_Character.StopFlying` _asbp_robot_dynamite)
  (`/Game/Robot_Dynamite/Base/BPML_Utilities.DisplayMessage` "Robot Dynamite feels heavy again" (struct :`R` 0.424385 :`G` 0.040803 :`B` 0.040803 :`A` 1.0)))

(event `NightVision`
  (bind _outactors (`GameplayStatics.GetAllActorsWithTag` "NightVision"))
  (for _array_element _outactors
    (bind _aspost_process_volume (cast `PostProcessVolume` _array_element))
    (set `PostProcessVolume.Settings` (make `PostProcessSettings` :`AmbientCubemapTint` (struct :`G` 1.0 :`B` 0.5 :`A` 1.0) :`AmbientCubemap` "/Game/Robot_Dynamite/Effects/Lighting/NightVision.NightVision") _aspost_process_volume)))

(event `NormalVision`
  (bind _outactors (`GameplayStatics.GetAllActorsWithTag` "NightVision"))
  (for _array_element _outactors
    (bind _aspost_process_volume (cast `PostProcessVolume` _array_element))
    (set `PostProcessVolume.Settings` (make `PostProcessSettings` :`AmbientCubemapIntensity` 0.0) _aspost_process_volume)))

(fn `UserConstructionScript`)