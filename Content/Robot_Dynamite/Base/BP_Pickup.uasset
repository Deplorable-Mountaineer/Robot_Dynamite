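; Base pickup actor that gives a BP_Character an item or reloads one it already holds, then destroys itself with a sound.
; On overlap it tries to grant the item at its Index, falling back to reload, or only reloads if ReloadOnly; a positive SuperAmount adds extra beyond the maximum.
; BeginPlay creates a gun inventory slot only under a Pawn parent actor, and that slot's item spawn never runs.
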(event OnComponentBeginOverlap(Collider)
  (params (OverlappedComponent :type Primitive%20Component%20Object%20Reference) (OtherActor :type Actor%20Object%20Reference) (OtherComp :type Primitive%20Component%20Object%20Reference) (OtherBodyIndex :type Integer) (bFromSweep :type Boolean) (SweepResult :type Hit%20Result%20Structure%20%28by%20ref%29))
  (bind _asbp_character (Utilities|Casting|CastToBP_Character OtherActor))
  (if (Variables|Config|GetbReloadOnly)
    (bind _success (CallFunction|TrytoReload _asbp_character))
    (CallFunction|DebugPrint false "Try to reload" "Reload Only" (Utilities|String|ToString(Boolean) _success))
    (if _success
      (Actor|DestroyActor :!label _label))
    (else
      (bind _success_2 (CallFunction|TrytoGet _asbp_character))
      (CallFunction|DebugPrint false "Try to Get" "Not Reload Only" (Utilities|String|ToString(Boolean) _success_2))
      (if _success_2
        (goto _label)
        (else
          (bind _success_3 (CallFunction|TrytoReload _asbp_character))
          (CallFunction|DebugPrint false "Try to reload" "Not Reload Only" (Utilities|String|ToString(Boolean) _success_3))
          (if _success_3
            (goto _label)))))))

(event EventDestroyed
  (Audio|PlaySoundatLocation (Variables|Config|GetPickupSound) (Transformation|GetWorldLocation (Variables|Default|GetDefaultSceneRoot))))

(event EventBeginPlay
  (CallFunction|CreateInventorySlot "/Game/Robot_Dynamite/Base/BP_Gun.BP_Gun_C" "Got  Item" "Using  Item" "Reloaded  Item" "/Game/Robot_Dynamite/Characters/Player/T_PlayerLogo_D.T_PlayerLogo_D" false true))

(fn ConstructionScript)

(fn CreateInventorySlot
  (params (ItemClass :type Actor%20Class%20Reference) (TextOnPickup :type String) (TextOnUse :type String) (TextOnReload :type String) (Image :type Texture%20Object%20Reference) (DiscardOnUse :type Boolean) (Reloadable :type Boolean))
  (bind _returnvalue (Actor|GetParentActor))
  (bind _aspawn (Utilities|Casting|CastToPawn _returnvalue))
  (bind _returnvalue_2 (Game|SpawnActorfromClass "/Game/Robot_Dynamite/Characters/BP_InventorySlot.BP_InventorySlot_C" (Math|Transform|MakeTransform "0, 0, 0") "AlwaysSpawn" _returnvalue ItemClass (stale _returnvalue) TextOnPickup TextOnUse TextOnReload Image DiscardOnUse Reloadable _aspawn))
  (bind _output_get (Variables|Default|SetInventorySlot _returnvalue_2))
  (return _output_get))

(fn TrytoReload
  (params (Character :type BP%20Character%20Object%20Reference))
  (bind _index (Variables|Config|GetIndex))
  (bind _superamount (Variables|Config|GetSuperAmount))
  (if (.True (Default|HasItem Character _index))
    (bind _amount (Class|BPIReloadable|GetAmount(Message) (Variables|/Game/Robot_Dynamite/Characters/BP_InventorySlot.BP_InventorySlot_C|GetItem (Variables|Default|GetInventorySlot))))
    (bind _bamountchanged (Class|BPIReloadable|Reload(Message) (Variables|/Game/Robot_Dynamite/Characters/BP_InventorySlot.BP_InventorySlot_C|GetItem (Default|GetInventorySlot Character _index)) (+ _amount _superamount) (> _superamount 0.0)))
    (CallFunction|DebugPrint false "Called Reload" (Utilities|String|ToString(Boolean) _bamountchanged))
    (return _bamountchanged)
    (else
      (return false))))

(fn TrytoGet
  (params (Character :type BP%20Character%20Object%20Reference))
  (bind _index (Variables|Config|GetIndex))
  (bind (_true _item _out_index) (Default|HasItem Character _index))
  (if _true
    (return false)
    (else
      (Default|GotNewItem Character _out_index)
      (return true))))