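; BP_Train is an environment actor that builds a train of a configurable number of identical cars.
; The construction script starts from the Car component and adds a static mesh component with the same mesh for each additional car.
; Each new car attaches to the previous one's "Next" socket, so the mesh's socket sets the spacing and orientation of the chain.
; The event graph holds no active logic.
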(fn `UserConstructionScript`
  (locals (CurrentCar :type "StaticMeshComponent Object Reference"))
  (set `local.CurrentCar` (`self.Car`))
  (for _ (range 2 (+ (`self.NumberOfCars`) 1))
    (bind _returnvalue (`AddComponent|NODE_AddStaticMeshComponent-0` :`bManualAttachment` true :`RelativeTransform` (`KismetMathLibrary.MakeTransform` (0.0 0.0 0.0))))
    (`SceneComponent.K2_AttachToComponent` _returnvalue (`local.CurrentCar`) "Next" "KeepRelative" "KeepRelative" "KeepRelative" true)
    (set `local.CurrentCar` _returnvalue)
    (`StaticMeshComponent.SetStaticMesh` _returnvalue (`StaticMeshComponent.StaticMesh` (`self.Car`)))))