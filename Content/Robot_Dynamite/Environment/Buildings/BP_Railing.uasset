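; BP_Railing is a railing building piece whose length is set by NumberOfSegments.
; Its construction script adds one static mesh component per segment, attached to the root and stepped along local Y.
; Odd-numbered segments are turned 180 degrees in yaw and shifted back along Y, so the mesh alternates facing along the run.
; The event graph has no active logic.
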(fn `UserConstructionScript`
  (for _index (range 1 (+ (`self.NumberOfSegments`) 1))
    (bind _returnvalue (mod _index 2))
    (bind _returnvalue_2 (`AddComponent|NODE_AddStaticMeshComponent-0` :`bManualAttachment` true :`RelativeTransform` (`KismetMathLibrary.MakeTransform` (`KismetMathLibrary.MakeVector` 0.0 (- (* _index 50.0) (* _returnvalue 47.5))) (`KismetMathLibrary.MakeRotator` 0.0 0.0 (* _returnvalue 180.0)))))
    (`SceneComponent.K2_AttachToComponent` _returnvalue_2 (`self.DefaultSceneRoot`) "None" "KeepRelative" "KeepRelative" "KeepRelative" true)))