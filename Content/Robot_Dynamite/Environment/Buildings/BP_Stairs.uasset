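; BP_Stairs is a procedural staircase building piece whose length is set by the NumSteps variable.
; Its construction script starts from the StairSegment mesh and adds one static mesh component per additional step, reusing the same mesh.
; Each new step attaches to the previous one's NextStep socket, so the socket on the mesh defines the rise and offset of the chain.
; The event graph has no active logic.
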(fn `UserConstructionScript`
  (locals (CurrentStep :type "StaticMeshComponent Object Reference"))
  (set `local.CurrentStep` (`self.StairSegment`))
  (for _ (range 2 (+ (`self.NumSteps`) 1))
    (bind _returnvalue (`AddComponent|NODE_AddStaticMeshComponent-0` :`bManualAttachment` true :`RelativeTransform` (`KismetMathLibrary.MakeTransform` (0.0 0.0 0.0))))
    (`SceneComponent.K2_AttachToComponent` _returnvalue (`local.CurrentStep`) "NextStep" "KeepRelative" "KeepRelative" "KeepRelative" true)
    (`StaticMeshComponent.SetStaticMesh` _returnvalue (`StaticMeshComponent.StaticMesh` (`local.CurrentStep`)))
    (set `local.CurrentStep` _returnvalue)))