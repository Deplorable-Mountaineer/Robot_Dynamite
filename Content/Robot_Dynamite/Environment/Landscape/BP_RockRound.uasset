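; BP_RockRound is a round rock landscape prop that varies its own appearance from a seed.
; The construction script derives a random stream from RandomSeed and passes it to Randomize, so each seed gives a repeatable result.
; Randomize sets the Rock component's world rotation including roll, a non-uniform scale within a bounded range, and a material picked from the Materials array.
; It has no runtime logic.
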(fn `Randomize`
  (params (Stream :type "RandomStream Structure (by ref)"))
  (bind _rock (`self.Rock`))
  (bind _materials (`self.Materials`))
  (`SceneComponent.K2_SetWorldRotation` _rock (`KismetMathLibrary.RandomRotatorFromStream` true Stream) false false)
  (`SceneComponent.SetWorldScale3D` _rock (`KismetMathLibrary.MakeVector` (`KismetMathLibrary.RandomFloatInRangeFromStream` 0.71 1.41 Stream) (`KismetMathLibrary.RandomFloatInRangeFromStream` 0.71 1.41 Stream) (`KismetMathLibrary.RandomFloatInRangeFromStream` 0.71 1.41 Stream)))
  (`PrimitiveComponent.SetMaterial` (`self.Rock`) 0 (`|GetArrayItem` _materials (`KismetMathLibrary.RandomIntegerInRangeFromStream` 0 (- (`KismetArrayLibrary.Array_Length` _materials) 1) Stream))))

(fn `UserConstructionScript`
  (`self.Randomize` (`KismetMathLibrary.MakeRandomStream` (`KismetMathLibrary.RandomIntegerFromStream` 1048576 (`KismetMathLibrary.MakeRandomStream` (`self.RandomSeed`))))))