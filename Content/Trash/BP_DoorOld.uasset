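; BP_DoorOld is a lockable door actor that auto-opens when its trigger is overlapped while unlocked.
; It subscribes to an optional UnlockSwitch, whose notifications lock or unlock it according to the BP_SwitchOld position.
; Lock changes and blocked open attempts display colored messages with the door's name.
; Tick runs a delayed auto-close that skips closing while pawns remain in the trigger; Open and Close only set a flag.
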(event `/Game/Robot_Dynamite/Base/BPI_Notify_Receiver.Notify`
  (params (Sender :type "Actor Object Reference"))
  (bind _returnvalue (>= (`/Game/Trash/BP_SwitchOld.GetCurrentPosition` (cast `/Game/Trash/BP_SwitchOld` Sender :!pure true)) 1))
  (if (`self.bLocked`)
    (if _returnvalue
      (`self.Unlock`))
    (elif (not _returnvalue)
      (`self.Lock`))))

(event `self.ReceiveBeginPlay`
  (bind _unlockswitch (`self.UnlockSwitch`))
  (`/Engine/EditorBlueprintResources/StandardMacros.IsValid` _unlockswitch
    (:`Is Valid`
      (`/Game/Trash/BP_SwitchOld.Subscribe` _unlockswitch self))))

(event `Open`
  (set `self.bOpen` true))

(event `Close`
  (set `self.bOpen` false))

(event `self.Trigger.OnComponentBeginOverlap`
  (params (OverlappedComponent :type "PrimitiveComponent Object Reference") (OtherActor :type "Actor Object Reference") (OtherComp :type "PrimitiveComponent Object Reference") (OtherBodyIndex :type Integer) (bFromSweep :type Boolean) (SweepResult :type "HitResult Structure (by ref)"))
  (`self.AutoOpen`))

(event `Lock`
  (set `self.bLocked` true)
  (`/Game/Robot_Dynamite/Base/BPML_Utilities_Actors.DisplayMessage` (`KismetStringLibrary.Concat_StrStr` (`self.Name In Game`) " is now locked!") (struct :`R` 0.424385 :`G` 0.040803 :`B` 0.040803 :`A` 1.0)))

(event `Unlock`
  (set `self.bLocked` false)
  (`/Game/Robot_Dynamite/Base/BPML_Utilities_Actors.DisplayMessage` (`KismetStringLibrary.Concat_StrStr` (`self.Name In Game`) " is now unlocked!")))

(event `OnAttemptOpenLocked`
  (`/Game/Robot_Dynamite/Base/BPML_Utilities_Actors.DisplayMessage` (`KismetStringLibrary.Concat_StrStr` (`self.Name In Game`) " is locked!") (struct :`R` 0.424385 :`G` 0.040803 :`B` 0.040803 :`A` 1.0)))

(event `AutoOpen`
  (if (or (`self.bOpen`) (`self.bLocked`))
    (if (`self.bLocked`)
      (`self.OnAttemptOpenLocked`))
    (else
      (`self.Open`))))

(event `self.ReceiveTick`
  (params (DeltaSeconds :type "Float (single-precision)"))
  (if (and (> (`self.Auto Close Delay`) 0.0) (`self.bOpen`))
    (`KismetSystemLibrary.Delay` (`self.Auto Close Delay`))
    (if (not (and (> (`KismetArrayLibrary.Array_Length` (`PrimitiveComponent.GetOverlappingActors` (`self.Trigger`) "/Script/Engine.Pawn")) 0) (`self.bOpen`)))
      (`self.Close`))))

(fn `UserConstructionScript`)