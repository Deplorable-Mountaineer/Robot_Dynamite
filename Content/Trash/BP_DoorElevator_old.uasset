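; An elevator door Blueprint, marked old, that slides a left and a right door between a closed position and open positions.
; Its construction script rebuilds each mover's waypoint list from child-actor BP_Waypoints: a shared closed point, then that side's open point.
; Open and Close call the parent logic, then step both movers to the next or previous waypoint.
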(event `self.ReceiveBeginPlay`
  (`parent.ReceiveBeginPlay`))

(event `self.Open`
  (`parent.Open`)
  (`/Game/Robot_Dynamite/Effects/Movement/BP_MoveToWaypoints.Next` (`self.MoveRightDoor`))
  (`/Game/Robot_Dynamite/Effects/Movement/BP_MoveToWaypoints.Next` (`self.MoveLeftDoor`)))

(event `self.Close`
  (`parent.Close`)
  (`/Game/Robot_Dynamite/Effects/Movement/BP_MoveToWaypoints.previous` (`self.MoveLeftDoor`))
  (`/Game/Robot_Dynamite/Effects/Movement/BP_MoveToWaypoints.previous` (`self.MoveRightDoor`)))

(fn `Set up Waypoints`
  (bind _waypoints (`/Game/Robot_Dynamite/Effects/Movement/BP_MoveToWaypoints.Waypoints` (`self.MoveLeftDoor`)))
  (bind _waypoints_2 (`/Game/Robot_Dynamite/Effects/Movement/BP_MoveToWaypoints.Waypoints` (`self.MoveRightDoor`)))
  (`KismetArrayLibrary.Array_Clear` (`/Game/Robot_Dynamite/Effects/Movement/BP_MoveToWaypoints.Waypoints` (`self.MoveRightDoor`)))
  (`KismetArrayLibrary.Array_Clear` (`/Game/Robot_Dynamite/Effects/Movement/BP_MoveToWaypoints.Waypoints` (`self.MoveLeftDoor`)))
  (bind _asbp_waypoint (cast `/Game/Robot_Dynamite/Effects/Movement/BP_Waypoint` (`ChildActorComponent.ChildActor` (`self.WaypointClosed`))))
  (`KismetArrayLibrary.Array_Add` _waypoints _asbp_waypoint)
  (bind _asbp_waypoint_2 (cast `/Game/Robot_Dynamite/Effects/Movement/BP_Waypoint` (`ChildActorComponent.ChildActor` (`self.WaypointOpenLeft`))))
  (`KismetArrayLibrary.Array_Add` _waypoints _asbp_waypoint_2)
  (bind _asbp_waypoint_3 (cast `/Game/Robot_Dynamite/Effects/Movement/BP_Waypoint` (`ChildActorComponent.ChildActor` (`self.WaypointClosed`))))
  (`KismetArrayLibrary.Array_Add` _waypoints_2 _asbp_waypoint_3)
  (bind _asbp_waypoint_4 (cast `/Game/Robot_Dynamite/Effects/Movement/BP_Waypoint` (`ChildActorComponent.ChildActor` (`self.WaypointOpenRight`))))
  (`KismetArrayLibrary.Array_Add` _waypoints_2 _asbp_waypoint_4))

(fn `UserConstructionScript`
  (`parent.UserConstructionScript`)
  (`self.Set up Waypoints`))