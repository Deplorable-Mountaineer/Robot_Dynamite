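; Light component whose brightness and color are controlled through float channels on a BP transceiver component.
; On BeginPlay it tunes in to brightness, hue and saturation channels, then applies their values once through SetLightProperties.
; Brightness can be read as a base-10 exponent for logarithmic control, and hue and saturation become an HSV color at full value.
; Missing channels fall back to fixed defaults.
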(event `self.ReceiveBeginPlay`
  (`/Game/Robot_Dynamite/Effects/Communication/BP_TransceiverComponent.Tune In Float` (`self.BP_TransceiverComponent`) (`self.Brightness Channel`))
  (`/Game/Robot_Dynamite/Effects/Communication/BP_TransceiverComponent.Tune In Float` (`self.BP_TransceiverComponent`) (`self.Hue Channel`))
  (`/Game/Robot_Dynamite/Effects/Communication/BP_TransceiverComponent.Tune In Float` (`self.BP_TransceiverComponent`) (`self.Saturation Channel`))
  (`self.SetLightProperties`))

(fn `SetLightProperties`
  (bind _bp_transceivercomponent (`self.BP_TransceiverComponent`))
  (`|ExecutionSequence`
    (:`then_0`
      (bind (_value _channel_exists) (`/Game/Robot_Dynamite/Effects/Communication/BP_TransceiverComponent.Receive Float` (`self.BP_TransceiverComponent`) (`self.Brightness Channel`)))
      (if _channel_exists
        (`self.SetIntensity` (select `bool` (`self.bLogarithmicBrightness`) :`false` _value :`true` (`KismetMathLibrary.MultiplyMultiply_FloatFloat` 10.0 _value)))
        (else
          (`self.SetIntensity` 3000.0))))
    (:`then_1`
      (bind (_value_2 _channel_exists_2) (`/Game/Robot_Dynamite/Effects/Communication/BP_TransceiverComponent.Receive Float` _bp_transceivercomponent (`self.Hue Channel`)))
      (bind (_value_3 _channel_exists_3) (`/Game/Robot_Dynamite/Effects/Communication/BP_TransceiverComponent.Receive Float` _bp_transceivercomponent (`self.Saturation Channel`)))
      (`self.SetLightColor` (`KismetMathLibrary.HSVToRGB` (select `bool` _channel_exists_2 :`false` 0.35 :`true` _value_2) (select `bool` _channel_exists_3 :`false` 0.25 :`true` _value_3) 1.0)))))