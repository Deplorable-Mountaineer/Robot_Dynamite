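; Swinging door Blueprint that opens and closes by stepping an OpenDoor waypoint component between closed and opened positions, extending its parent's open and close logic.
; The construction script rebuilds the waypoint list from two child actor waypoints, WaypointClosed and WaypointOpened.
; On BeginPlay, it sets the opened waypoint's yaw to OpenAngle, so the swing angle comes from a single variable.
; Open advances to the next waypoint and Close returns to the previous one.
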(event `self.ReceiveBeginPlay`
  (`SceneComponent.K2_SetRelativeRotation` (`Actor.RootComponent` (`|GetArrayItem` (`/Game/Robot_Dynamite/Effects/Movement/BP_MoveToWaypoints.Waypoints` (`self.OpenDoor`)) 1)) (`KismetMathLibrary.MakeRotator` 0.0 0.0 (`self.OpenAngle`)) false false))

(event `self.Open`
  (`parent.Open`)
  (`/Game/Robot_Dynamite/Effects/Movement/BP_MoveToWaypoints.Next` (`self.OpenDoor`)))

(event `self.Close`
  (`parent.Close`)
  (`/Game/Robot_Dynamite/Effects/Movement/BP_MoveToWaypoints.previous` (`self.OpenDoor`)))

(fn `UserConstructionScript`
  (bind _waypoints (`/Game/Robot_Dynamite/Effects/Movement/BP_MoveToWaypoints.Waypoints` (`self.OpenDoor`)))
  (`parent.UserConstructionScript`)
  (`KismetArrayLibrary.Array_Clear` _waypoints)
  (`KismetArrayLibrary.Array_Add` _waypoints (cast `/Game/Robot_Dynamite/Effects/Movement/BP_Waypoint` (`ChildActorComponent.ChildActor` (`self.Waypoint_Closed`)) :!pure true))
  (`KismetArrayLibrary.Array_Add` _waypoints (cast `/Game/Robot_Dynamite/Effects/Movement/BP_Waypoint` (`ChildActorComponent.ChildActor` (`self.Waypoint_Opened`)) :!pure true)))