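; Despite its name, BP_ControllableLight is a two-panel door whose openness is driven by a float received on a transceiver channel.
; Tick moves the open amount toward that target over OpenTime, lerping each panel between closed and open sockets on the frame.
; If a panel hits a BP_Character while not nearly closed, the door reopens, then restores the channel value after a delay.
; Construction and BeginPlay reset the pose, tune the channel and label it on both sides.
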(event `self.ReceiveBeginPlay`
  (`self.Reset`))

(event `self.ReceiveTick`
  (params (DeltaSeconds :type "Float (single-precision)"))
  (bind _returnvalue (/ DeltaSeconds (`self.Open Time`)))
  (if (not (`KismetMathLibrary.NearlyEqual_FloatFloat` (`self.Open Amount`) (`self.New Open Amount`)))
    (if (< (`self.Open Amount`) (`self.New Open Amount`))
      (set `self.Open Amount` (+ (`self.Open Amount`) _returnvalue))
      (if (not (< (`self.Open Amount`) (`self.New Open Amount`)))
        (set `self.Open Amount` (`self.New Open Amount`)))
      (else
        (set `self.Open Amount` (- (`self.Open Amount`) _returnvalue))
        (if (< (`self.Open Amount`) (`self.New Open Amount`))
          (set `self.Open Amount` (`self.New Open Amount`)))))
    (`self.AdjustDoorOpenness`)))

(event `self.BP_Transceiver.Float Received`
  (bind (_value _channel_exists) (`/Game/Robot_Dynamite/Effects/Communication/BP_TransceiverComponent.Receive Float` (`self.BP_Transceiver`) (`self.Input Channel`)))
  (if _channel_exists
    (set `self.New Open Amount` _value)))

(event `self.LeftDoor.OnComponentHit`
  (params (HitComponent :type "PrimitiveComponent Object Reference") (OtherActor :type "Actor Object Reference") (OtherComp :type "PrimitiveComponent Object Reference") (NormalImpulse :type "Vector Structure") (Hit :type "HitResult Structure (by ref)"))
  ;[1 0.2783 0] Safety Auto Reopen When Blocked By Character
  (cast `/Game/Robot_Dynamite/Characters/BP_Character` OtherActor)
  (if (>= (`self.Open Amount`) 0.1) :!label _label
    (set `self.New Open Amount` 1.0)
    (`KismetSystemLibrary.Delay` (`self.Open Time`))
    (bind (_value _channel_exists) (`/Game/Robot_Dynamite/Effects/Communication/BP_TransceiverComponent.Receive Float` (`self.BP_Transceiver`) (`self.Input Channel`)))
    (if _channel_exists
      (set `self.New Open Amount` _value))))

(event `self.RightDoor.OnComponentHit`
  (params (HitComponent :type "PrimitiveComponent Object Reference") (OtherActor :type "Actor Object Reference") (OtherComp :type "PrimitiveComponent Object Reference") (NormalImpulse :type "Vector Structure") (Hit :type "HitResult Structure (by ref)"))
  ;[1 0.2783 0] Safety Auto Reopen When Blocked By Character
  (cast `/Game/Robot_Dynamite/Characters/BP_Character` OtherActor)
  (goto _label))

(fn `AdjustDoorOpenness`
  (bind _frame (`self.Frame`))
  (bind _open_amount (`self.Open Amount`))
  (`SceneComponent.K2_SetWorldTransform` (`self.LeftDoor`) (`KismetMathLibrary.TLerp` (`SceneComponent.GetSocketTransform` _frame "Left Door Closed" "RTS_World") (`SceneComponent.GetSocketTransform` _frame "Left Door Open" "RTS_World") _open_amount) false false)
  (`SceneComponent.K2_SetWorldTransform` (`self.RightDoor`) (`KismetMathLibrary.TLerp` (`SceneComponent.GetSocketTransform` _frame "Right Door Closed" "RTS_World") (`SceneComponent.GetSocketTransform` _frame "Right Door Open" "RTS_World") _open_amount) false false))

(fn `Reset`
  (bind _returnvalue (`KismetTextLibrary.Conv_NameToText` (`self.Input Channel`)))
  (set `self.Open Amount` (`self.New Open Amount`))
  (`self.AdjustDoorOpenness`)
  (`/Game/Robot_Dynamite/Effects/Communication/BP_TransceiverComponent.Tune In Float` (`self.BP_Transceiver`) (`self.Input Channel`))
  (`TextRenderComponent.K2_SetText` (`self.In Channel Text`) _returnvalue)
  (`TextRenderComponent.K2_SetText` (`self.In Channel Text Other Side`) _returnvalue))

(fn `UserConstructionScript`
  (`self.Reset`))