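; BP_Preview is a display actor that shows a single material on preview meshes alongside a text label with its name.
; The construction script applies the Material variable to several slots of the Base component and to the first slot of the Preview component.
; It then sets the TextRender text to the material's display name.
; The event graph holds only disabled placeholder events, so the actor has no runtime logic.
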(fn `UserConstructionScript`
  (bind _base (`self.Base`))
  (bind _material (`self.Material`))
  (`PrimitiveComponent.SetMaterial` _base 3 _material)
  (`PrimitiveComponent.SetMaterial` _base 6 _material)
  (`PrimitiveComponent.SetMaterial` _base 7 _material)
  (`PrimitiveComponent.SetMaterial` _base 8 _material)
  (`PrimitiveComponent.SetMaterial` _base 9 _material)
  (`PrimitiveComponent.SetMaterial` (`self.preview`) 0 _material)
  (`TextRenderComponent.SetText` (`self.TextRender`) (`KismetSystemLibrary.GetDisplayName` _material)))